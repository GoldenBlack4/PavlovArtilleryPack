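; Smoke artillery projectile that ignores its owning actor in movement collision and expires after a short lifespan.
; On collision hit, the server applies direct damage to the struck actor only, triggers a multicast for effects, then destroys the projectile.
; The multicast spawns fire and smoke emitters, near and distant explosion sounds, and a temporary decal sized from the outer explosion radius sphere.
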(event OnComponentHit(Collision)
  (params (HitComponent :type Primitive%20Component%20Object%20Reference) (OtherActor :type Actor%20Object%20Reference) (OtherComp :type Primitive%20Component%20Object%20Reference) (NormalImpulse :type Vector :default "0, 0, 0") (Hit :type Hit%20Result%20Structure%20%28by%20ref%29))
  (bind (_bblockinghit _binitialoverlap _time _distance _location _impactpoint _normal _impactnormal _physmat _hitactor) (Collision|BreakHitResult Hit))
  (Networking|SwitchHasAuthority
    (:Authority
      (Game|Damage|ApplyDamage _hitactor 8e+01 (Game|GetInstigatorController) self)
      (CallFunction|FXMulticast _impactpoint HitComponent _normal)
      (Actor|DestroyActor))))

(event Custom|FX_Multicast
  (params (Location :type Vector) (AttachToComponent :type Scene%20Component%20Object%20Reference) (Normal :type Vector))
  (Effects|SpawnEmitteratLocation (Variables|Default|GetFireEmitter) Location "0, 0, 0" "0.500000,0.500000,0.500000")
  (Effects|SpawnEmitteratLocation (Variables|Default|GetSmokeEmitter) Location)
  (Audio|PlaySoundatLocation (Variables|Default|GetBulletExplosion) Location "0, 0, 0" 0.5 1.0 0.0 0 0 0)
  (Rendering|Decal|SpawnDecalatLocation (Variables|Default|GetExplosionDecal) (Math|Conversions|ToVector(Float) (Components|Sphere|GetScaledSphereRadius (Variables|Default|GetOuterExplosionRadius))) Location (Math|Rotator|MakeRotfromX Normal) 1e+01)
  (Audio|PlaySoundatLocation (Variables|Default|GetBulletDistantExplosion) Location "0, 0, 0" 0.2 2.0 0.0 0 0 0))

(event EventBeginPlay
  (Collision|IgnoreActorwhenMoving (Variables|Default|GetCollision) self true)
  (Actor|SetLifeSpan 1e+01))

(fn ConstructionScript)