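; Pavlov artillery pack spawner that keeps one artillery shell item available at its own transform.
; From BeginPlay it runs an endless authority-only loop, polling each second while the spawned shell reference is still valid.
; Once that reference is invalid, it waits RespawnDelay, spawns a new shell through the game logic's SpawnItemWRef and stores it, retrying after failures.
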(event EventBeginPlay
  (Networking|SwitchHasAuthority :!label _label
    (:Authority
      (Utilities|IsValid (Variables|Default|GetSpawnedPavlovShell)
        (:Is%20Valid
          (Utilities|FlowControl|Delay 1.0)
          (goto _label))
        (:Is%20Not%20Valid
          (Utilities|FlowControl|Delay (Variables|Default|GetRespawnDelay))
          (bind (_bsuccessful _item) (Class|PavlovGameLogic|SpawnItemWRef (Class|PavlovLibrary|GetGameLogic) (Utilities|Struct|MakePavlovItemSpawnParams "artilleryshell" 0 false false 0 true (Transformation|GetActorTransform) false true)))
          (if _bsuccessful
            (Variables|Default|SetSpawnedPavlovShell _item)
            (goto _label)
            (else
              (goto _label))))))))

(fn ConstructionScript)