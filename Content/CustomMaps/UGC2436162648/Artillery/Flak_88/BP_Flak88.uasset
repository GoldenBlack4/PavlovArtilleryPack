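; Flak 88 artillery gun for Pavlov that players aim, load and fire through interact boxes replicated via HandProxy.
; Shells load by overlap; the trap must close to fire a BP_ArtilleryProjectile, then open to eject the casing.
; Aiming toggles delay-driven rotation loops with a safety timeout, animating wheels, plus pistons for elevation.
; Explosive damage, matched by causer name, swaps in a wreck and respawn spawner; debug keys and a fire loop aid testing.
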(event OnInteractBoxServer(Pavlov_Fire)
  (params (InteractType :type EInteractType%20Enum :default "Grabbed") (HandProxy :type Pavlov%20Hand%20Proxy%20Object%20Reference) (InteractBox :type Pavlov%20Interact%20Box%20Object%20Reference))
  (bind _flak_cannon (Variables|Components|GetFlak_Cannon))
  (bind _returnvalue (Transformation|GetSocketTransform _flak_cannon "FireSocket" "RTS_World"))
  ;[1 0.5647 0.7758] Firing
  (if (Variables|ActionDONOTEDITTHOSE|GetIsLoaded)
    (if (Variables|ActionDONOTEDITTHOSE|GetTrapClosed)
      (CallFunction|PlayFireFX)
      (CallFunction|FireAnimation)
      (Variables|ActionDONOTEDITTHOSE|SetIsLoaded false)
      (Variables|ActionDONOTEDITTHOSE|SetHasFired true)
      (Variables|ActionDONOTEDITTHOSE|SetHasEmptyShell true)
      (Game|SpawnActorfromClass "/Game/CustomMaps/UGC2436162648/Artillery/Common/Projectiles/BP_ArtilleryProjectile.BP_ArtilleryProjectile_C" (Math|Transform|MakeTransform (.location _returnvalue) (.rotation _returnvalue) "0.180000,0.180000,0.180000") "AlwaysSpawn" 0 "/Game/CustomMaps/UGC2436162648/Artillery/Common/Sound/grenade_explo_Cue.grenade_explo_Cue" "/Game/CustomMaps/UGC2436162648/Artillery/Common/Sound/Explosiondistant_Cue.Explosiondistant_Cue" "/Game/CustomMaps/UGC2436162648/Artillery/Common/Decals/T_Impact.T_Impact" (Game|GetInstigator (Components|GetOwner HandProxy))))))

(event OnInteractBoxClient(Pavlov_RotateUp)
  (params (InteractType :type EInteractType%20Enum :default "Grabbed") (HandProxy :type Pavlov%20Hand%20Proxy%20Object%20Reference) (InteractBox :type Pavlov%20Interact%20Box%20Object%20Reference))
  ;[1 1 1] Interaction Pavlov Replication
  (Class|PavlovHandProxy|ReplicateInteractServer HandProxy InteractType InteractBox))

(event OnInteractBoxClient(Pavlov_RotateDown)
  (params (InteractType :type EInteractType%20Enum :default "Grabbed") (HandProxy :type Pavlov%20Hand%20Proxy%20Object%20Reference) (InteractBox :type Pavlov%20Interact%20Box%20Object%20Reference))
  ;[1 1 1] Interaction Pavlov Replication
  (Class|PavlovHandProxy|ReplicateInteractServer HandProxy InteractType InteractBox))

(event OnInteractBoxServer(Pavlov_RotateDown)
  (params (InteractType :type EInteractType%20Enum :default "Grabbed") (HandProxy :type Pavlov%20Hand%20Proxy%20Object%20Reference) (InteractBox :type Pavlov%20Interact%20Box%20Object%20Reference))
  (bind _flak_gunbarrel (Variables|Components|GetFlak_GunBarrel))
  ;[0.8025 1 0.6847] Controls
  ;;[1 1 1] Y Movement
  (if (Variables|MovementDONOTEDITTHOSE|GetGB_DO_Stop)
    (CallFunction|AutoStop)
    (if (Variables|MovementDONOTEDITTHOSE|GetGB_UP_Stop)
      _
      (else
        (Variables|MovementDONOTEDITTHOSE|SetGB_UP_Stop true)))
    (Variables|MovementDONOTEDITTHOSE|SetGB_DO_Stop false)
    (CallFunction|PlayRotationSound)
    (if (not (Variables|MovementDONOTEDITTHOSE|GetGB_DO_Stop)) :!label _label
      (if (>= (.pitch (Variables|/Script/Engine.SceneComponent|GetRelativeRotation _flak_gunbarrel)) 5.0)
        (Variables|MovementDONOTEDITTHOSE|SetGB_DO_Stop true)
        (CallFunction|StopRotationSound)
        (else
          (Transformation|AddLocalRotation _flak_gunbarrel (Math|Rotator|MakeRotator 0.0 (Variables|MovementDONOTEDITTHOSE|GetGunBarrelDegree) 0.0) false false)
          (Utilities|FlowControl|Delay (Variables|MovementDONOTEDITTHOSE|GetGunBarrelSpeed))
          (CallFunction|MovePistonsBackward)
          (CallFunction|RotateWheelYDown)
          (goto _label))))
    (else
      (Variables|MovementDONOTEDITTHOSE|SetGB_DO_Stop true)
      (Variables|MovementDONOTEDITTHOSE|SetGB_UP_Stop true)
      (CallFunction|StopRotationSound))))

(event OnInteractBoxServer(Pavlov_RotateUp)
  (params (InteractType :type EInteractType%20Enum :default "Grabbed") (HandProxy :type Pavlov%20Hand%20Proxy%20Object%20Reference) (InteractBox :type Pavlov%20Interact%20Box%20Object%20Reference))
  (bind _flak_gunbarrel (Variables|Components|GetFlak_GunBarrel))
  ;[0.8025 1 0.6847] Controls
  ;;[1 1 1] Y Movement
  (if (Variables|MovementDONOTEDITTHOSE|GetGB_UP_Stop)
    (CallFunction|AutoStop)
    (if (Variables|MovementDONOTEDITTHOSE|GetGB_DO_Stop)
      _
      (else
        (Variables|MovementDONOTEDITTHOSE|SetGB_DO_Stop true)))
    (Variables|MovementDONOTEDITTHOSE|SetGB_UP_Stop false)
    (CallFunction|PlayRotationSound)
    (if (not (Variables|MovementDONOTEDITTHOSE|GetGB_UP_Stop)) :!label _label
      (if (<= (.pitch (Variables|/Script/Engine.SceneComponent|GetRelativeRotation _flak_gunbarrel)) -7e+01)
        (Variables|MovementDONOTEDITTHOSE|SetGB_UP_Stop true)
        (CallFunction|StopRotationSound)
        (else
          (Transformation|AddLocalRotation _flak_gunbarrel (Math|Rotator|MakeRotator 0.0 (* (Variables|MovementDONOTEDITTHOSE|GetGunBarrelDegree) -1.0) 0.0) false false)
          (Utilities|FlowControl|Delay (Variables|MovementDONOTEDITTHOSE|GetGunBarrelSpeed))
          (CallFunction|MovePistonsForward)
          (CallFunction|RotateWheelYUp)
          (goto _label))))
    (else
      (Variables|MovementDONOTEDITTHOSE|SetGB_UP_Stop true)
      (Variables|MovementDONOTEDITTHOSE|SetGB_DO_Stop true)
      (CallFunction|StopRotationSound))))

(event OnInteractBoxServer(Pavlov_RotateRight)
  (params (InteractType :type EInteractType%20Enum :default "Grabbed") (HandProxy :type Pavlov%20Hand%20Proxy%20Object%20Reference) (InteractBox :type Pavlov%20Interact%20Box%20Object%20Reference))
  ;[0.8025 1 0.6847] Controls
  ;;[1 1 1] Z Movement
  (if (Variables|MovementDONOTEDITTHOSE|GetDR_R_Stop)
    (CallFunction|AutoStop)
    (if (Variables|MovementDONOTEDITTHOSE|GetDR_L_Stop)
      _
      (else
        (Variables|MovementDONOTEDITTHOSE|SetDR_L_Stop true)))
    (Variables|MovementDONOTEDITTHOSE|SetDR_R_Stop false)
    (CallFunction|PlayRotationSound)
    (if (Variables|MovementDONOTEDITTHOSE|GetDR_R_Stop) :!label _label
      (CallFunction|StopRotationSound)
      (else
        (Transformation|AddLocalRotation (Variables|Components|GetFlak_Dock) (Math|Rotator|MakeRotator 0.0 0.0 (Variables|MovementDONOTEDITTHOSE|GetDockRotateDegree)) false false)
        (Utilities|FlowControl|Delay (Variables|MovementDONOTEDITTHOSE|GetDockRotateSpeed))
        (CallFunction|RotateWheelZLeft)
        (goto _label)))
    (else
      (Variables|MovementDONOTEDITTHOSE|SetDR_R_Stop true)
      (Variables|MovementDONOTEDITTHOSE|SetDR_L_Stop true)
      (CallFunction|StopRotationSound))))

(event OnInteractBoxServer(Pavlov_RotateLeft)
  (params (InteractType :type EInteractType%20Enum :default "Grabbed") (HandProxy :type Pavlov%20Hand%20Proxy%20Object%20Reference) (InteractBox :type Pavlov%20Interact%20Box%20Object%20Reference))
  ;[0.8025 1 0.6847] Controls
  ;;[1 1 1] Z Movement
  (if (Variables|MovementDONOTEDITTHOSE|GetDR_L_Stop)
    (CallFunction|AutoStop)
    (if (Variables|MovementDONOTEDITTHOSE|GetDR_R_Stop)
      _
      (else
        (Variables|MovementDONOTEDITTHOSE|SetDR_R_Stop true)))
    (Variables|MovementDONOTEDITTHOSE|SetDR_L_Stop false)
    (CallFunction|PlayRotationSound)
    (if (Variables|MovementDONOTEDITTHOSE|GetDR_L_Stop) :!label _label
      (CallFunction|StopRotationSound)
      (else
        (Transformation|AddLocalRotation (Variables|Components|GetFlak_Dock) (Math|Rotator|MakeRotator 0.0 0.0 (* (Variables|MovementDONOTEDITTHOSE|GetDockRotateDegree) -1.0)) false false)
        (Utilities|FlowControl|Delay (Variables|MovementDONOTEDITTHOSE|GetDockRotateSpeed))
        (CallFunction|RotateWheelZRight)
        (goto _label)))
    (else
      (Variables|MovementDONOTEDITTHOSE|SetDR_L_Stop true)
      (Variables|MovementDONOTEDITTHOSE|SetDR_R_Stop true)
      (CallFunction|StopRotationSound))))

(event OnComponentBeginOverlap(Pavlov_Loading)
  (params (OverlappedComponent :type Primitive%20Component%20Object%20Reference) (OtherActor :type Actor%20Object%20Reference) (OtherComp :type Primitive%20Component%20Object%20Reference) (OtherBodyIndex :type Integer) (bFromSweep :type Boolean) (SweepResult :type Hit%20Result%20Structure%20%28by%20ref%29))
  ;[1 0.5647 0.7758] Loading
  (Networking|SwitchHasAuthority
    (:Authority
      (bind _ascustom_item_shell (Utilities|Casting|CastToCustomItem_Shell OtherActor))
      (Utilities|IsValid _ascustom_item_shell
        (:Is%20Valid
          (Utilities|CanReload?
            (:Yes
              (Default|DestroyAfterLoading _ascustom_item_shell)
              (Variables|ActionDONOTEDITTHOSE|SetIsLoaded true)
              (CallFunction|PlayShellLoadSound))))))))

(event OnComponentBeginOverlap(WidgetsVisibility)
  (params (OverlappedComponent :type Primitive%20Component%20Object%20Reference) (OtherActor :type Actor%20Object%20Reference) (OtherComp :type Primitive%20Component%20Object%20Reference) (OtherBodyIndex :type Integer) (bFromSweep :type Boolean) (SweepResult :type Hit%20Result%20Structure%20%28by%20ref%29))
  ;[1 1 1] Widgets Visibility
  (Development|SetHiddeninGame (Variables|Components|GetArrowDown) false false))

(event OnComponentEndOverlap(WidgetsVisibility)
  (params (OverlappedComponent :type Primitive%20Component%20Object%20Reference) (OtherActor :type Actor%20Object%20Reference) (OtherComp :type Primitive%20Component%20Object%20Reference) (OtherBodyIndex :type Integer))
  ;[1 1 1] Widgets Visibility
  (Development|SetHiddeninGame (Variables|Components|GetArrowDown) true false))

(event OnInteractBoxClient(Pavlov_Fire)
  (params (InteractType :type EInteractType%20Enum :default "Grabbed") (HandProxy :type Pavlov%20Hand%20Proxy%20Object%20Reference) (InteractBox :type Pavlov%20Interact%20Box%20Object%20Reference))
  ;[1 1 1] Interaction Pavlov Replication
  (Class|PavlovHandProxy|ReplicateInteractServer HandProxy InteractType InteractBox))

(event OnInteractBoxClient(Pavlov_Trap)
  (params (InteractType :type EInteractType%20Enum :default "Grabbed") (HandProxy :type Pavlov%20Hand%20Proxy%20Object%20Reference) (InteractBox :type Pavlov%20Interact%20Box%20Object%20Reference))
  ;[1 1 1] Interaction Pavlov Replication
  (Class|PavlovHandProxy|ReplicateInteractServer HandProxy InteractType InteractBox))

(event OnInteractBoxClient(Pavlov_Loading)
  (params (InteractType :type EInteractType%20Enum :default "Grabbed") (HandProxy :type Pavlov%20Hand%20Proxy%20Object%20Reference) (InteractBox :type Pavlov%20Interact%20Box%20Object%20Reference))
  ;[1 1 1] Interaction Pavlov Replication
  (Class|PavlovHandProxy|ReplicateInteractServer HandProxy InteractType InteractBox))

(event OnInteractBoxServer(Pavlov_Trap)
  (params (InteractType :type EInteractType%20Enum :default "Grabbed") (HandProxy :type Pavlov%20Hand%20Proxy%20Object%20Reference) (InteractBox :type Pavlov%20Interact%20Box%20Object%20Reference))
  ;[1 0.5647 0.7758] Loading
  (if (Variables|ActionDONOTEDITTHOSE|GetTrapClosed)
    (Variables|ActionDONOTEDITTHOSE|SetHasEmptyShell false)
    (CallFunction|UnloadAmmAnim)
    (CallFunction|LeverAnimUnload)
    (Variables|ActionDONOTEDITTHOSE|SetTrapClosed false)
    (CallFunction|PlayTrapSound)
    (if (Variables|ActionDONOTEDITTHOSE|GetHasFired)
      (CallFunction|ShellEjecting)
      (Variables|ActionDONOTEDITTHOSE|SetHasFired false))
    (else
      (CallFunction|AmmAnim)
      (CallFunction|LeverAnim)
      (Variables|ActionDONOTEDITTHOSE|SetTrapClosed true)
      (CallFunction|PlayTrapSound))))

(event OnInteractBoxClient(Pavlov_Reload)
  (params (InteractType :type EInteractType%20Enum :default "Grabbed") (HandProxy :type Pavlov%20Hand%20Proxy%20Object%20Reference) (InteractBox :type Pavlov%20Interact%20Box%20Object%20Reference))
  ;[1 1 1] Interaction Pavlov Replication
  (Class|PavlovHandProxy|ReplicateInteractServer HandProxy InteractType InteractBox))

(event OnInteractBoxClient(Pavlov_RotateLeft)
  (params (InteractType :type EInteractType%20Enum :default "Grabbed") (HandProxy :type Pavlov%20Hand%20Proxy%20Object%20Reference) (InteractBox :type Pavlov%20Interact%20Box%20Object%20Reference))
  ;[1 1 1] Interaction Pavlov Replication
  (Class|PavlovHandProxy|ReplicateInteractServer HandProxy InteractType InteractBox))

(event OnInteractBoxClient(Pavlov_RotateRight)
  (params (InteractType :type EInteractType%20Enum :default "Grabbed") (HandProxy :type Pavlov%20Hand%20Proxy%20Object%20Reference) (InteractBox :type Pavlov%20Interact%20Box%20Object%20Reference))
  ;[1 1 1] Interaction Pavlov Replication
  (Class|PavlovHandProxy|ReplicateInteractServer HandProxy InteractType InteractBox))

(event Custom|FireLoop
  ;[1 0.1094 0.1094] DEBUG
  (CallFunction|TestreloadClient)
  (CallFunction|TesttrapClient)
  (Utilities|FlowControl|Delay 1.0)
  (CallFunction|Testfire))

(event Custom|PlayFireFX
  (bind _flak_cannon (Variables|Components|GetFlak_Cannon))
  (bind _returnvalue (Transformation|GetSocketTransform _flak_cannon "FireSocket" "RTS_World"))
  ;[1 0.823 0.4892] FX
  (Effects|SpawnEmitteratLocation (Variables|EditableVariables|GetFiringEmitter) (.location _returnvalue) (.rotation _returnvalue) "0.500000,0.500000,0.500000")
  (Audio|PlaySoundatLocation (Variables|EditableVariables|GetFiringSound) (.location _returnvalue) "0, 0, 0" 1.0 1.0 0.0 "/Game/CustomMaps/UGC2436162648/Artillery/Common/Sound/SA_Antitankgun.SA_Antitankgun" 0 0))

(event Custom|FireAnimation
  (bind _cannoninitlocation (Variables|AnimationDONOTEDITTHOSE|GetCannonInitLocation))
  ;[0.2874 0.9131 1] Fire Animation
  (bind _newtrack_1 (Timeline|Timeline_3 PlayFromStart)
    (:Update
      (Transformation|SetRelativeLocation (Variables|Components|GetFlak_Cannon) (Math|Vector|Lerp(Vector) _cannoninitlocation (+ _cannoninitlocation "50.000000, 0, 0") _newtrack_1) false false))))

(event Custom|RotateWheelYDown
  ;[0.2874 0.9131 1] Wheels Animation
  (Transformation|AddLocalRotation (Variables|Components|GetFlak_WheelLeft) (Math|Rotator|MakeRotator 0.0 (* (Variables|AnimationDONOTEDITTHOSE|GetWheelSpeed) -1.0) 0.0) false false))

(event Custom|LeverAnim
  (bind _leverinitrotation (Variables|AnimationDONOTEDITTHOSE|GetLeverInitRotation))
  (bind (_roll _pitch _yaw) (Math|Rotator|BreakRotator _leverinitrotation))
  ;[0.2874 0.9131 1] Reload Animation
  ;;[1 1 1] Lever
  (bind _newtrack_1 (Timeline|Timeline_1 PlayFromStart)
    (:Update
      (Transformation|SetRelativeRotation (Variables|Components|GetFlak_Lever) (Math|Rotator|Lerp(Rotator) _leverinitrotation (Math|Rotator|MakeRotator _roll _pitch (+ _yaw -9e+01)) _newtrack_1) false false))))

(event Custom|MovePistonsBackward
  ;[0.2874 0.9131 1] Pistons Animation
  (Transformation|AddLocalOffset (Variables|Components|GetFlak_Pistons) (Math|Vector|MakeVector (Variables|AnimationDONOTEDITTHOSE|GetPistonsSpeed) 0.0 0.0) false false))

(event Custom|LeverAnimUnload
  (bind _leverinitrotation (Variables|AnimationDONOTEDITTHOSE|GetLeverInitRotation))
  (bind (_roll _pitch _yaw) (Math|Rotator|BreakRotator _leverinitrotation))
  ;[0.2874 0.9131 1] Reload Animation
  ;;[1 1 1] Lever
  (bind _newtrack_1 (Timeline|Timeline_1 Reverse)
    (:Update
      (Transformation|SetRelativeRotation (Variables|Components|GetFlak_Lever) (Math|Rotator|Lerp(Rotator) _leverinitrotation (Math|Rotator|MakeRotator _roll _pitch (+ _yaw -9e+01)) _newtrack_1) false false))))

(event Custom|ActivateFireLoop
  ;[1 0.1094 0.1094] DEBUG
  (bind _returnvalue (Utilities|Time|SetTimerbyEvent (delegate Custom|FireLoop) 2.0 true)))

(event Custom|DeactivateFireLoop
  ;[1 0.1094 0.1094] DEBUG
  (Utilities|Time|PauseTimerbyHandle (stale Custom|ActivateFireLoop _returnvalue)))

(event Custom|ReactivateFireLoop
  ;[1 0.1094 0.1094] DEBUG
  (Utilities|Time|UnpauseTimerbyHandle (stale Custom|ActivateFireLoop _returnvalue)))

(event Custom|ShellEjecting
  (bind _pavlov_loading (Variables|Components|GetPavlov_Loading))
  ;[0.2874 0.9131 1] Shell Emitter
  (Utilities|FlowControl|Delay 0.5)
  (Rendering|SetVisibility (Variables|Components|GetShellCaseMesh) false true)
  (Effects|SpawnEmitteratLocation "/Game/CustomMaps/UGC2436162648/Artillery/Common/Particles/PS_ShellParticle.PS_ShellParticle" (Transformation|GetWorldLocation _pavlov_loading) (Transformation|GetWorldRotation _pavlov_loading)))

(event Custom|PlayShellLoadSound
  ;[1 0.823 0.4892] FX
  (Audio|PlaySoundatLocation (Variables|EditableVariables|GetShellLoadingSound) (.location (Transformation|GetSocketTransform (Variables|Components|GetFlak_Ammunition) "None" "RTS_World")) "0, 0, 0" 1.0 1.0 0.0 "/Game/CustomMaps/UGC2436162648/Artillery/Common/Sound/SA_Close.SA_Close" 0 0))

(event Custom|AutoStopTimer
  ;[0.8025 1 0.6847] Controls
  ;;[1 1 1] AutoStop Security
  (Variables|MovementDONOTEDITTHOSE|SetDR_R_Stop true)
  (Variables|MovementDONOTEDITTHOSE|SetGB_UP_Stop true)
  (Variables|MovementDONOTEDITTHOSE|SetDR_L_Stop true)
  (Variables|MovementDONOTEDITTHOSE|SetGB_DO_Stop true))

(event Custom|testtrap_Client
  ;[1 0.5647 0.7758] Loading
  (if (Variables|ActionDONOTEDITTHOSE|GetTrapClosed)
    (Variables|ActionDONOTEDITTHOSE|SetHasEmptyShell false)
    (CallFunction|UnloadAmmAnim)
    (CallFunction|LeverAnimUnload)
    (Variables|ActionDONOTEDITTHOSE|SetTrapClosed false)
    (CallFunction|PlayTrapSound)
    (if (Variables|ActionDONOTEDITTHOSE|GetHasFired)
      (CallFunction|ShellEjecting)
      (Variables|ActionDONOTEDITTHOSE|SetHasFired false))
    (else
      (CallFunction|AmmAnim)
      (CallFunction|LeverAnim)
      (Variables|ActionDONOTEDITTHOSE|SetTrapClosed true)
      (CallFunction|PlayTrapSound))))

(event Custom|testfire
  (bind _flak_cannon (Variables|Components|GetFlak_Cannon))
  (bind _returnvalue (Transformation|GetSocketTransform _flak_cannon "FireSocket" "RTS_World"))
  ;[1 0.5647 0.7758] Firing
  (if (Variables|ActionDONOTEDITTHOSE|GetIsLoaded)
    (if (Variables|ActionDONOTEDITTHOSE|GetTrapClosed)
      (CallFunction|PlayFireFX)
      (CallFunction|FireAnimation)
      (Variables|ActionDONOTEDITTHOSE|SetIsLoaded false)
      (Variables|ActionDONOTEDITTHOSE|SetHasFired true)
      (Variables|ActionDONOTEDITTHOSE|SetHasEmptyShell true)
      (Game|SpawnActorfromClass "/Game/CustomMaps/UGC2436162648/Artillery/Common/Projectiles/BP_ArtilleryProjectile.BP_ArtilleryProjectile_C" (Math|Transform|MakeTransform (.location _returnvalue) (.rotation _returnvalue) "0.180000,0.180000,0.180000") "AlwaysSpawn" 0 "/Game/CustomMaps/UGC2436162648/Artillery/Common/Sound/grenade_explo_Cue.grenade_explo_Cue" "/Game/CustomMaps/UGC2436162648/Artillery/Common/Sound/Explosiondistant_Cue.Explosiondistant_Cue" "/Game/CustomMaps/UGC2436162648/Artillery/Common/Decals/T_Impact.T_Impact" (Game|GetInstigator (Components|GetOwner (stale OnInteractBoxServer(Pavlov_Fire) HandProxy)))))))

(event Custom|testrotatedown
  (bind _flak_gunbarrel (Variables|Components|GetFlak_GunBarrel))
  ;[0.8025 1 0.6847] Controls
  ;;[1 1 1] Y Movement
  (if (Variables|MovementDONOTEDITTHOSE|GetGB_DO_Stop)
    (CallFunction|AutoStop)
    (if (Variables|MovementDONOTEDITTHOSE|GetGB_UP_Stop)
      _
      (else
        (Variables|MovementDONOTEDITTHOSE|SetGB_UP_Stop true)))
    (Variables|MovementDONOTEDITTHOSE|SetGB_DO_Stop false)
    (CallFunction|PlayRotationSound)
    (if (not (Variables|MovementDONOTEDITTHOSE|GetGB_DO_Stop)) :!label _label
      (if (>= (.pitch (Variables|/Script/Engine.SceneComponent|GetRelativeRotation _flak_gunbarrel)) 5.0)
        (Variables|MovementDONOTEDITTHOSE|SetGB_DO_Stop true)
        (CallFunction|StopRotationSound)
        (else
          (Transformation|AddLocalRotation _flak_gunbarrel (Math|Rotator|MakeRotator 0.0 (Variables|MovementDONOTEDITTHOSE|GetGunBarrelDegree) 0.0) false false)
          (Utilities|FlowControl|Delay (Variables|MovementDONOTEDITTHOSE|GetGunBarrelSpeed))
          (CallFunction|MovePistonsBackward)
          (CallFunction|RotateWheelYDown)
          (goto _label))))
    (else
      (Variables|MovementDONOTEDITTHOSE|SetGB_DO_Stop true)
      (Variables|MovementDONOTEDITTHOSE|SetGB_UP_Stop true)
      (CallFunction|StopRotationSound))))

(event Custom|testrotateup
  (bind _flak_gunbarrel (Variables|Components|GetFlak_GunBarrel))
  ;[0.8025 1 0.6847] Controls
  ;;[1 1 1] Y Movement
  (if (Variables|MovementDONOTEDITTHOSE|GetGB_UP_Stop)
    (CallFunction|AutoStop)
    (if (Variables|MovementDONOTEDITTHOSE|GetGB_DO_Stop)
      _
      (else
        (Variables|MovementDONOTEDITTHOSE|SetGB_DO_Stop true)))
    (Variables|MovementDONOTEDITTHOSE|SetGB_UP_Stop false)
    (CallFunction|PlayRotationSound)
    (if (not (Variables|MovementDONOTEDITTHOSE|GetGB_UP_Stop)) :!label _label
      (if (<= (.pitch (Variables|/Script/Engine.SceneComponent|GetRelativeRotation _flak_gunbarrel)) -7e+01)
        (Variables|MovementDONOTEDITTHOSE|SetGB_UP_Stop true)
        (CallFunction|StopRotationSound)
        (else
          (Transformation|AddLocalRotation _flak_gunbarrel (Math|Rotator|MakeRotator 0.0 (* (Variables|MovementDONOTEDITTHOSE|GetGunBarrelDegree) -1.0) 0.0) false false)
          (Utilities|FlowControl|Delay (Variables|MovementDONOTEDITTHOSE|GetGunBarrelSpeed))
          (CallFunction|MovePistonsForward)
          (CallFunction|RotateWheelYUp)
          (goto _label))))
    (else
      (Variables|MovementDONOTEDITTHOSE|SetGB_UP_Stop true)
      (Variables|MovementDONOTEDITTHOSE|SetGB_DO_Stop true)
      (CallFunction|StopRotationSound))))

(event Custom|testrotateleft
  ;[0.8025 1 0.6847] Controls
  ;;[1 1 1] Z Movement
  (if (Variables|MovementDONOTEDITTHOSE|GetDR_L_Stop)
    (CallFunction|AutoStop)
    (if (Variables|MovementDONOTEDITTHOSE|GetDR_R_Stop)
      _
      (else
        (Variables|MovementDONOTEDITTHOSE|SetDR_R_Stop true)))
    (Variables|MovementDONOTEDITTHOSE|SetDR_L_Stop false)
    (CallFunction|PlayRotationSound)
    (if (Variables|MovementDONOTEDITTHOSE|GetDR_L_Stop) :!label _label
      (CallFunction|StopRotationSound)
      (else
        (Transformation|AddLocalRotation (Variables|Components|GetFlak_Dock) (Math|Rotator|MakeRotator 0.0 0.0 (* (Variables|MovementDONOTEDITTHOSE|GetDockRotateDegree) -1.0)) false false)
        (Utilities|FlowControl|Delay (Variables|MovementDONOTEDITTHOSE|GetDockRotateSpeed))
        (CallFunction|RotateWheelZRight)
        (goto _label)))
    (else
      (Variables|MovementDONOTEDITTHOSE|SetDR_L_Stop true)
      (Variables|MovementDONOTEDITTHOSE|SetDR_R_Stop true)
      (CallFunction|StopRotationSound))))

(event Custom|PlayRotationSound
  ;[1 0.823 0.4892] FX
  (Audio|Components|Audio|Play (Variables|Default|GetAudio) 0.0))

(event Custom|testdebug_fireloop
  ;[1 0.1094 0.1094] DEBUG
  (CallFunction|ActivateFireLoop)
  (CallFunction|ReactivateFireLoop))

(event Custom|testreload_client
  ;[1 0.5647 0.7758] Loading
  (Utilities|CanReload?
    (:Yes
      (Variables|ActionDONOTEDITTHOSE|SetIsLoaded true)
      (CallFunction|PlayShellLoadSound))))

(event Custom|MovePistonsForward
  ;[0.2874 0.9131 1] Pistons Animation
  (Transformation|AddLocalOffset (Variables|Components|GetFlak_Pistons) (Math|Vector|MakeVector (* (Variables|AnimationDONOTEDITTHOSE|GetPistonsSpeed) -1.0) 0.0 0.0) false false))

(event Custom|RotateWheelYUp
  ;[0.2874 0.9131 1] Wheels Animation
  (Transformation|AddLocalRotation (Variables|Components|GetFlak_WheelLeft) (Math|Rotator|MakeRotator 0.0 (Variables|AnimationDONOTEDITTHOSE|GetWheelSpeed) 0.0) false false))

(event Custom|StopRotationSound
  ;[1 0.823 0.4892] FX
  (if (Math|Boolean|ANDBoolean (Variables|MovementDONOTEDITTHOSE|GetDR_R_Stop) (Variables|MovementDONOTEDITTHOSE|GetDR_L_Stop) (Variables|MovementDONOTEDITTHOSE|GetGB_UP_Stop) (Variables|MovementDONOTEDITTHOSE|GetGB_DO_Stop))
    (Audio|Components|Audio|Stop (Variables|Default|GetAudio))))

(event Custom|RotateWheelZLeft
  ;[0.2874 0.9131 1] Wheels Animation
  (Transformation|AddLocalRotation (Variables|Components|GetFlak_WheelRight) (Math|Rotator|MakeRotator 0.0 (Variables|AnimationDONOTEDITTHOSE|GetWheelSpeed) 0.0) false false))

(event Custom|testdebug_client
  ;[1 0.1094 0.1094] DEBUG
  (Utilities|FlowControl|MultiGate false true -1
    (:Out%200
      (Variables|Debug|SetDEBUG true)
      (Variables|Debug|SetHiddeBoxes false))
    (:Out%201
      (Variables|Debug|SetDEBUG false)
      (Variables|Debug|SetHiddeBoxes true)))
  (Development|SetHiddeninGame (Variables|Components|GetPavlov_Loading) (Variables|Debug|GetHiddeBoxes) false))

(event Custom|testdebug_stopfireloop
  ;[1 0.1094 0.1094] DEBUG
  (CallFunction|DeactivateFireLoop))

(event Custom|EnableInput_Client
  ;[0.6417 0.5249 1] BeginPlay
  (Input|EnableInput (Game|GetPlayerController 0)))

(event Custom|testrotateright
  ;[0.8025 1 0.6847] Controls
  ;;[1 1 1] Z Movement
  (if (Variables|MovementDONOTEDITTHOSE|GetDR_R_Stop)
    (CallFunction|AutoStop)
    (if (Variables|MovementDONOTEDITTHOSE|GetDR_L_Stop)
      _
      (else
        (Variables|MovementDONOTEDITTHOSE|SetDR_L_Stop true)))
    (Variables|MovementDONOTEDITTHOSE|SetDR_R_Stop false)
    (CallFunction|PlayRotationSound)
    (if (Variables|MovementDONOTEDITTHOSE|GetDR_R_Stop) :!label _label
      (CallFunction|StopRotationSound)
      (else
        (Transformation|AddLocalRotation (Variables|Components|GetFlak_Dock) (Math|Rotator|MakeRotator 0.0 0.0 (Variables|MovementDONOTEDITTHOSE|GetDockRotateDegree)) false false)
        (Utilities|FlowControl|Delay (Variables|MovementDONOTEDITTHOSE|GetDockRotateSpeed))
        (CallFunction|RotateWheelZLeft)
        (goto _label)))
    (else
      (Variables|MovementDONOTEDITTHOSE|SetDR_R_Stop true)
      (Variables|MovementDONOTEDITTHOSE|SetDR_L_Stop true)
      (CallFunction|StopRotationSound))))

(event Custom|RotateWheelZRight
  ;[0.2874 0.9131 1] Wheels Animation
  (Transformation|AddLocalRotation (Variables|Components|GetFlak_WheelRight) (Math|Rotator|MakeRotator 0.0 (Variables|AnimationDONOTEDITTHOSE|GetWheelSpeed) 0.0) false false))

(event Custom|PlayTrapSound
  ;[1 0.823 0.4892] FX
  (Audio|PlaySoundatLocation (Variables|EditableVariables|GetTrapSound) (.location (Transformation|GetSocketTransform (Variables|Components|GetFlak_Ammunition) "None" "RTS_World")) "0, 0, 0" 1.0 1.0 0.0 "/Game/CustomMaps/UGC2436162648/Artillery/Common/Sound/SA_Close.SA_Close" 0 0))

(event Custom|AutoStop
  ;[0.8025 1 0.6847] Controls
  ;;[1 1 1] AutoStop Security
  (Utilities|Time|SetTimerbyEvent (delegate Custom|AutoStopTimer) 15.0))

(event Custom|AmmAnim
  (bind _trapinitlocation (Variables|AnimationDONOTEDITTHOSE|GetTrapInitLocation))
  ;[0.2874 0.9131 1] Reload Animation
  ;;[1 1 1] Ammunition Trap
  (bind _newtrack_1 (Timeline|Timeline_0 PlayFromStart)
    (:Update
      (Transformation|SetRelativeLocation (Variables|Components|GetFlak_Ammunition) (Math|Vector|Lerp(Vector) _trapinitlocation (+ _trapinitlocation "0,15.000000,0.000000") _newtrack_1) false false))))

(event Custom|UnloadAmmAnim
  (bind _trapinitlocation (Variables|AnimationDONOTEDITTHOSE|GetTrapInitLocation))
  ;[0.2874 0.9131 1] Reload Animation
  ;;[1 1 1] Ammunition Trap
  (bind _newtrack_1 (Timeline|Timeline_0 Reverse)
    (:Update
      (Transformation|SetRelativeLocation (Variables|Components|GetFlak_Ammunition) (Math|Vector|Lerp(Vector) _trapinitlocation (+ _trapinitlocation "0,15.000000,0.000000") _newtrack_1) false false))))

(event EventBeginPlay
  ;[0.6417 0.5249 1] BeginPlay
  (Networking|SwitchHasAuthority
    (:Authority
      (Variables|Health|SetCurrentHealth (Variables|Health|GetMaxHealth))
      (Variables|Health|SetInitialSpawnTransform (Transformation|GetActorTransform))
      (Variables|AnimationDONOTEDITTHOSE|SetCannonInitLocation (Variables|/Script/Engine.SceneComponent|GetRelativeLocation (Variables|Components|GetFlak_Cannon)))
      (Variables|AnimationDONOTEDITTHOSE|SetTrapInitLocation (Variables|/Script/Engine.SceneComponent|GetRelativeLocation (Variables|Components|GetFlak_Ammunition)))
      (Variables|AnimationDONOTEDITTHOSE|SetLeverInitRotation (Variables|/Script/Engine.SceneComponent|GetRelativeRotation (Variables|Components|GetFlak_Lever)))
      (if (Variables|Debug|GetInputEnabled?)
        (CallFunction|EnableInputClient))
      (Variables|ActionDONOTEDITTHOSE|SetIsLoaded true)
      (Variables|ActionDONOTEDITTHOSE|SetTrapClosed false)
      (if (Variables|Debug|GetDEBUG_FireLoopBegin)
        (CallFunction|ActivateFireLoop)))))

(event Game|Damage|EventAnyDamage
  (params (Damage :type Float%20%28single-precision%29) (DamageType :type Damage%20Type%20Object%20Reference) (InstigatedBy :type Controller%20Object%20Reference) (DamageCauser :type Actor%20Object%20Reference))
  (bind _returnvalue (Utilities|GetDisplayName DamageCauser))
  ;[1 0.1269 0] Damage System
  (if (Math|Boolean|ORBoolean (Utilities|String|StartsWith _returnvalue "Rocket") (Utilities|String|StartsWith _returnvalue "Grenade_") (Utilities|String|StartsWith _returnvalue "Shell_") (Utilities|String|StartsWith _returnvalue "BP_ArtilleryProjectile") (Utilities|String|StartsWith _returnvalue "CI_GammonBomb"))
    (Variables|Health|SetCurrentHealth (- (Variables|Health|GetCurrentHealth) Damage))
    (if (<= (Variables|Health|GetCurrentHealth) 0.0)
      (bind _returnvalue_2 (Game|SpawnActorfromClass "/Game/CustomMaps/UGC2436162648/Artillery/Flak_88/BP_Flak88_Destroyed.BP_Flak88_Destroyed_C" (Transformation|GetActorTransform) "AlwaysSpawn" 0 0))
      (Default|SpawnDestroyed _returnvalue_2)
      (bind _returnvalue_3 (Game|SpawnActorfromClass "/Game/CustomMaps/UGC2436162648/Artillery/Flak_88/Flak88_Spawner.Flak88_Spawner_C" (Variables|Health|GetInitialSpawnTransform) "Undefined" 0 (Variables|Health|GetRespawnDelay) (Variables|Health|GetMaxHealth) false false 0))
      (Variables|/Game/CustomMaps/UGC2436162648/Artillery/Flak_88/Flak88_Spawner.Flak88_Spawner_C|SetDestroyedMesh _returnvalue_3 _returnvalue_2)
      (Actor|DestroyActor))))

(event Input|KeyboardEvents|9
  (params (Key :type Key%20Structure))
  ;[1 0.1094 0.1094] DEBUG
  ;;[1 1 1] Editor Controls
  (:Pressed
    (CallFunction|TestdebugStopfireloop)))

(event Input|KeyboardEvents|8
  (params (Key :type Key%20Structure))
  ;[1 0.1094 0.1094] DEBUG
  ;;[1 1 1] Editor Controls
  (:Pressed
    (CallFunction|TestdebugFireloop)))

(event Input|KeyboardEvents|Up
  (params (Key :type Key%20Structure))
  ;[1 0.1094 0.1094] DEBUG
  ;;[1 1 1] Editor Controls
  (:Pressed
    (CallFunction|Testrotateup)))

(event Input|KeyboardEvents|Down
  (params (Key :type Key%20Structure))
  ;[1 0.1094 0.1094] DEBUG
  ;;[1 1 1] Editor Controls
  (:Pressed
    (CallFunction|Testrotatedown)))

(event Input|KeyboardEvents|0
  (params (Key :type Key%20Structure))
  ;[1 0.1094 0.1094] DEBUG
  ;;[1 1 1] Editor Controls
  (:Pressed
    (CallFunction|TestdebugClient)))

(event Input|KeyboardEvents|1
  (params (Key :type Key%20Structure))
  ;[1 0.1094 0.1094] DEBUG
  ;;[1 1 1] Editor Controls
  (:Pressed
    (CallFunction|Testfire)))

(event Input|KeyboardEvents|2
  (params (Key :type Key%20Structure))
  ;[1 0.1094 0.1094] DEBUG
  ;;[1 1 1] Editor Controls
  (:Pressed
    (CallFunction|TesttrapClient)))

(event Input|KeyboardEvents|3
  (params (Key :type Key%20Structure))
  ;[1 0.1094 0.1094] DEBUG
  ;;[1 1 1] Editor Controls
  (:Pressed
    (CallFunction|TestreloadClient)))

(event Input|KeyboardEvents|Left
  (params (Key :type Key%20Structure))
  ;[1 0.1094 0.1094] DEBUG
  ;;[1 1 1] Editor Controls
  (:Pressed
    (CallFunction|Testrotateleft)))

(event Input|KeyboardEvents|Right
  (params (Key :type Key%20Structure))
  ;[1 0.1094 0.1094] DEBUG
  ;;[1 1 1] Editor Controls
  (:Pressed
    (CallFunction|Testrotateright)))

(fn ConstructionScript)

(fn OnRepIsLoaded
  (bind _shellmesh (Variables|Components|GetShellMesh))
  (bind _shellcasemesh (Variables|Components|GetShellCaseMesh))
  (if (Variables|ActionDONOTEDITTHOSE|GetIsLoaded)
    (Rendering|SetVisibility _shellmesh true true)
    (Rendering|SetVisibility _shellcasemesh false true)
    (else
      (Rendering|SetVisibility _shellmesh false true)
      (Rendering|SetVisibility _shellcasemesh true true))))