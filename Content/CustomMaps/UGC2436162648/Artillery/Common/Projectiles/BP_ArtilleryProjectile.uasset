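; Artillery shell projectile that explodes on impact and self-expires after a short lifespan if it hits nothing.
; On hit, the server applies radial falloff damage sized by inner and outer explosion sphere components, plus direct damage to the struck actor, then destroys the projectile.
; A multicast event plays the explosion emitter, near and distant sounds, and a ground decal scaled to the outer radius.
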(event OnComponentHit(Collision)
  (params (HitComponent :type Primitive%20Component%20Object%20Reference) (OtherActor :type Actor%20Object%20Reference) (OtherComp :type Primitive%20Component%20Object%20Reference) (NormalImpulse :type Vector :default "0, 0, 0") (Hit :type Hit%20Result%20Structure%20%28by%20ref%29))
  (bind (_bblockinghit _binitialoverlap _time _distance _location _impactpoint _normal _impactnormal _physmat _hitactor) (Collision|BreakHitResult Hit))
  (bind _returnvalue (Game|GetInstigatorController))
  (bind _self self)
  (Networking|SwitchHasAuthority
    (:Authority
      (Class|GameplayStatics|ApplyRadialDamagewithFalloff 5e+02 8e+01 (Transformation|GetActorLocation) (Components|Sphere|GetScaledSphereRadius (Variables|Default|GetInnerExplosionRadius)) (Components|Sphere|GetScaledSphereRadius (Variables|Default|GetOuterExplosionRadius)) 0.5 0 0 _self _returnvalue "ECC_Visibility")
      (Game|Damage|ApplyDamage _hitactor 5e+02 _returnvalue _self)
      (CallFunction|FXMulticast _impactpoint)
      (Actor|DestroyActor))))

(event Custom|FX_Multicast
  (params (Location :type Vector))
  (Effects|SpawnEmitteratLocation "/Game/CustomMaps/UGC2436162648/Artillery/Common/Particles/Particles/Explosion/P_Firing.P_Firing" Location "0, 0, 0" "2.000000,2.000000,2.000000")
  (Audio|PlaySoundatLocation (Variables|Default|GetBulletExplosion) Location "0, 0, 0" 1.0 1.0 0.0 0 0 0)
  (Rendering|Decal|SpawnDecalatLocation (Variables|Default|GetExplosionDecal) (Math|Conversions|ToVector(Float) (Components|Sphere|GetScaledSphereRadius (Variables|Default|GetOuterExplosionRadius))) Location (Math|Rotator|MakeRotator 0.0 -9e+01 0.0) 1e+01)
  (Audio|PlaySoundatLocation (Variables|Default|GetBulletDistantExplosion) Location "0, 0, 0" 1.0 1.0 0.0 0 0 0))

(event EventBeginPlay
  (Collision|IgnoreActorwhenMoving (Variables|Default|GetCollision) self true)
  (Actor|SetLifeSpan 1e+01))

(fn ConstructionScript)