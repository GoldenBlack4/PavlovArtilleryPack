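; Crewed Pak 40 artillery gun for Pavlov, with destruction and optional timed respawn.
; Interact boxes replicate through HandProxy to server events that toggle delay-looped, clamped aiming with auto-stop, work the breech and fire BP_ArtilleryProjectile.
; Overlapping shell items load the gun through breech-state checks, with OnRep_IsLoaded swapping shell visuals.
; Damage is filtered by causer name prefix, boosting tank hits, and keyboard test events support debugging.
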(event OnInteractBoxServer(Pavlov_Fire)
  (params (InteractType :type EInteractType%20Enum :default "Grabbed") (HandProxy :type Pavlov%20Hand%20Proxy%20Object%20Reference) (InteractBox :type Pavlov%20Interact%20Box%20Object%20Reference))
  (bind _pak_cannon (Variables|Components|GetPak_Cannon))
  (bind _returnvalue (Transformation|GetSocketTransform _pak_cannon "FireSocket" "RTS_World"))
  ;[1 0.5647 0.7758] Firing
  (if (Variables|ActionDONOTEDITTHOSE|GetIsLoaded)
    (if (Variables|ActionDONOTEDITTHOSE|GetTrapClosed)
      (CallFunction|PlayFireFX)
      (CallFunction|FireAnimation)
      (Variables|ActionDONOTEDITTHOSE|SetIsLoaded false)
      (Variables|ActionDONOTEDITTHOSE|SetHasFired true)
      (Variables|ActionDONOTEDITTHOSE|SetHasEmptyShell true)
      (Game|SpawnActorfromClass "/Game/CustomMaps/UGC2436162648/Artillery/Common/Projectiles/BP_ArtilleryProjectile.BP_ArtilleryProjectile_C" (Math|Transform|MakeTransform (.location _returnvalue) (.rotation _returnvalue) "0.180000,0.180000,0.180000") "AlwaysSpawn" 0 "/Game/CustomMaps/UGC2436162648/Artillery/Common/Sound/grenade_explo_Cue.grenade_explo_Cue" "/Game/CustomMaps/UGC2436162648/Artillery/Common/Sound/Explosiondistant_Cue.Explosiondistant_Cue" "/Game/CustomMaps/UGC2436162648/Artillery/Common/Decals/T_Impact.T_Impact" (Game|GetInstigator (Components|GetOwner HandProxy))))))

(event OnInteractBoxClient(Pavlov_RotateUp)
  (params (InteractType :type EInteractType%20Enum :default "Grabbed") (HandProxy :type Pavlov%20Hand%20Proxy%20Object%20Reference) (InteractBox :type Pavlov%20Interact%20Box%20Object%20Reference))
  ;[1 1 1] Interaction Pavlov Replication
  (Class|PavlovHandProxy|ReplicateInteractServer HandProxy InteractType InteractBox))

(event OnInteractBoxClient(Pavlov_RotateDown)
  (params (InteractType :type EInteractType%20Enum :default "Grabbed") (HandProxy :type Pavlov%20Hand%20Proxy%20Object%20Reference) (InteractBox :type Pavlov%20Interact%20Box%20Object%20Reference))
  ;[1 1 1] Interaction Pavlov Replication
  (Class|PavlovHandProxy|ReplicateInteractServer HandProxy InteractType InteractBox))

(event OnInteractBoxServer(Pavlov_RotateDown)
  (params (InteractType :type EInteractType%20Enum :default "Grabbed") (HandProxy :type Pavlov%20Hand%20Proxy%20Object%20Reference) (InteractBox :type Pavlov%20Interact%20Box%20Object%20Reference))
  (bind _pak_rail (Variables|Components|GetPak_Rail))
  ;[0.8025 1 0.6847] Controls
  ;;[1 1 1] Y Movement
  (if (Variables|MovementDONOTEDITTHOSE|GetGB_DO_Stop)
    (CallFunction|AutoStop)
    (if (Variables|MovementDONOTEDITTHOSE|GetGB_UP_Stop)
      _
      (else
        (Variables|MovementDONOTEDITTHOSE|SetGB_UP_Stop true)))
    (Variables|MovementDONOTEDITTHOSE|SetGB_DO_Stop false)
    (if (not (Variables|MovementDONOTEDITTHOSE|GetGB_DO_Stop)) :!label _label
      (if (>= (.roll (Variables|/Script/Engine.SceneComponent|GetRelativeRotation _pak_rail)) 2.0)
        (Variables|MovementDONOTEDITTHOSE|SetGB_DO_Stop true)
        (else
          (Transformation|AddLocalRotation _pak_rail (Math|Rotator|MakeRotator (Variables|MovementDONOTEDITTHOSE|GetGunBarrelYDegree) 0.0 0.0) false false)
          (Utilities|FlowControl|Delay (Variables|MovementDONOTEDITTHOSE|GetGunBarrelYSpeed))
          (CallFunction|RotateWheelYDown)
          (CallFunction|PlayRotationSound)
          (goto _label))))
    (else
      (Variables|MovementDONOTEDITTHOSE|SetGB_DO_Stop true)
      (Variables|MovementDONOTEDITTHOSE|SetGB_UP_Stop true))))

(event OnInteractBoxServer(Pavlov_RotateUp)
  (params (InteractType :type EInteractType%20Enum :default "Grabbed") (HandProxy :type Pavlov%20Hand%20Proxy%20Object%20Reference) (InteractBox :type Pavlov%20Interact%20Box%20Object%20Reference))
  (bind _pak_rail (Variables|Components|GetPak_Rail))
  ;[0.8025 1 0.6847] Controls
  ;;[1 1 1] Y Movement
  (if (Variables|MovementDONOTEDITTHOSE|GetGB_UP_Stop)
    (CallFunction|AutoStop)
    (if (Variables|MovementDONOTEDITTHOSE|GetGB_DO_Stop)
      _
      (else
        (Variables|MovementDONOTEDITTHOSE|SetGB_DO_Stop true)))
    (Variables|MovementDONOTEDITTHOSE|SetGB_UP_Stop false)
    (if (not (Variables|MovementDONOTEDITTHOSE|GetGB_UP_Stop)) :!label _label
      (if (<= (.roll (Variables|/Script/Engine.SceneComponent|GetRelativeRotation _pak_rail)) -7.0)
        (Variables|MovementDONOTEDITTHOSE|SetGB_UP_Stop true)
        (else
          (Transformation|AddLocalRotation _pak_rail (Math|Rotator|MakeRotator (* (Variables|MovementDONOTEDITTHOSE|GetGunBarrelYDegree) -1.0) 0.0 0.0) false false)
          (Utilities|FlowControl|Delay (Variables|MovementDONOTEDITTHOSE|GetGunBarrelYSpeed))
          (CallFunction|RotateWheelYUp)
          (CallFunction|PlayRotationSound)
          (goto _label))))
    (else
      (Variables|MovementDONOTEDITTHOSE|SetGB_UP_Stop true)
      (Variables|MovementDONOTEDITTHOSE|SetGB_DO_Stop true))))

(event OnInteractBoxServer(Pavlov_RotateRight)
  (params (InteractType :type EInteractType%20Enum :default "Grabbed") (HandProxy :type Pavlov%20Hand%20Proxy%20Object%20Reference) (InteractBox :type Pavlov%20Interact%20Box%20Object%20Reference))
  ;[0.8025 1 0.6847] Controls
  ;;[1 1 1] Z Movement
  (if (Variables|MovementDONOTEDITTHOSE|GetDR_R_Stop)
    (CallFunction|AutoStop)
    (if (Variables|MovementDONOTEDITTHOSE|GetDR_L_Stop)
      _
      (else
        (Variables|MovementDONOTEDITTHOSE|SetDR_L_Stop true)))
    (Variables|MovementDONOTEDITTHOSE|SetDR_R_Stop false)
    (if (not (Variables|MovementDONOTEDITTHOSE|GetDR_R_Stop)) :!label _label
      (if (>= (.yaw (Variables|/Script/Engine.SceneComponent|GetRelativeRotation (Variables|Components|GetPak_Turret))) 25.0)
        (Variables|MovementDONOTEDITTHOSE|SetDR_R_Stop true)
        (else
          (Transformation|AddLocalRotation (Variables|Components|GetPak_Turret) (Math|Rotator|MakeRotator 0.0 0.0 (Variables|MovementDONOTEDITTHOSE|GetDockRotateZDegree)) false false)
          (Utilities|FlowControl|Delay (Variables|MovementDONOTEDITTHOSE|GetDockRotateZSpeed))
          (CallFunction|RotateWheelZLeft)
          (CallFunction|PlayRotationSound)
          (goto _label))))
    (else
      (Variables|MovementDONOTEDITTHOSE|SetDR_R_Stop true)
      (Variables|MovementDONOTEDITTHOSE|SetDR_L_Stop true))))

(event OnInteractBoxServer(Pavlov_RotateLeft)
  (params (InteractType :type EInteractType%20Enum :default "Grabbed") (HandProxy :type Pavlov%20Hand%20Proxy%20Object%20Reference) (InteractBox :type Pavlov%20Interact%20Box%20Object%20Reference))
  (bind _pak_turret (Variables|Components|GetPak_Turret))
  ;[0.8025 1 0.6847] Controls
  ;;[1 1 1] Z Movement
  (if (Variables|MovementDONOTEDITTHOSE|GetDR_L_Stop)
    (CallFunction|AutoStop)
    (if (Variables|MovementDONOTEDITTHOSE|GetDR_R_Stop)
      _
      (else
        (Variables|MovementDONOTEDITTHOSE|SetDR_R_Stop true)))
    (Variables|MovementDONOTEDITTHOSE|SetDR_L_Stop false)
    (if (not (Variables|MovementDONOTEDITTHOSE|GetDR_L_Stop)) :!label _label
      (if (<= (.yaw (Variables|/Script/Engine.SceneComponent|GetRelativeRotation _pak_turret)) -25.0)
        (Variables|MovementDONOTEDITTHOSE|SetDR_L_Stop true)
        (else
          (Transformation|AddLocalRotation _pak_turret (Math|Rotator|MakeRotator 0.0 0.0 (* (Variables|MovementDONOTEDITTHOSE|GetDockRotateZDegree) -1.0)) false false)
          (Utilities|FlowControl|Delay (Variables|MovementDONOTEDITTHOSE|GetDockRotateZSpeed))
          (CallFunction|RotateWheelZRight)
          (CallFunction|PlayRotationSound)
          (goto _label))))
    (else
      (Variables|MovementDONOTEDITTHOSE|SetDR_L_Stop true)
      (Variables|MovementDONOTEDITTHOSE|SetDR_R_Stop true))))

(event OnComponentBeginOverlap(Pavlov_Loading)
  (params (OverlappedComponent :type Primitive%20Component%20Object%20Reference) (OtherActor :type Actor%20Object%20Reference) (OtherComp :type Primitive%20Component%20Object%20Reference) (OtherBodyIndex :type Integer) (bFromSweep :type Boolean) (SweepResult :type Hit%20Result%20Structure%20%28by%20ref%29))
  ;[1 0.5647 0.7758] Loading
  (Networking|SwitchHasAuthority
    (:Authority
      (bind _ascustom_item_shell (Utilities|Casting|CastToCustomItem_Shell OtherActor))
      (Utilities|IsValid _ascustom_item_shell
        (:Is%20Valid
          (Utilities|CanReload?
            (:Yes
              (Default|RespawnAfterLoading _ascustom_item_shell)
              (Variables|ActionDONOTEDITTHOSE|SetIsLoaded true)
              (CallFunction|PlayShellLoadSound))))))))

(event OnInteractBoxClient(Pavlov_Fire)
  (params (InteractType :type EInteractType%20Enum :default "Grabbed") (HandProxy :type Pavlov%20Hand%20Proxy%20Object%20Reference) (InteractBox :type Pavlov%20Interact%20Box%20Object%20Reference))
  ;[1 1 1] Interaction Pavlov Replication
  (Class|PavlovHandProxy|ReplicateInteractServer HandProxy InteractType InteractBox))

(event OnInteractBoxClient(Pavlov_Trap)
  (params (InteractType :type EInteractType%20Enum :default "Grabbed") (HandProxy :type Pavlov%20Hand%20Proxy%20Object%20Reference) (InteractBox :type Pavlov%20Interact%20Box%20Object%20Reference))
  ;[1 1 1] Interaction Pavlov Replication
  (Class|PavlovHandProxy|ReplicateInteractServer HandProxy InteractType InteractBox))

(event OnInteractBoxClient(Pavlov_Loading)
  (params (InteractType :type EInteractType%20Enum :default "Grabbed") (HandProxy :type Pavlov%20Hand%20Proxy%20Object%20Reference) (InteractBox :type Pavlov%20Interact%20Box%20Object%20Reference))
  ;[1 1 1] Interaction Pavlov Replication
  (Class|PavlovHandProxy|ReplicateInteractServer HandProxy InteractType InteractBox))

(event OnInteractBoxServer(Pavlov_Trap)
  (params (InteractType :type EInteractType%20Enum :default "Grabbed") (HandProxy :type Pavlov%20Hand%20Proxy%20Object%20Reference) (InteractBox :type Pavlov%20Interact%20Box%20Object%20Reference))
  ;[1 0.5647 0.7758] Loading
  (if (Variables|ActionDONOTEDITTHOSE|GetTrapClosed)
    (Variables|ActionDONOTEDITTHOSE|SetHasEmptyShell false)
    (CallFunction|UnloadAmmAnim)
    (CallFunction|LeverAnimUnload)
    (Variables|ActionDONOTEDITTHOSE|SetTrapClosed false)
    (CallFunction|PlayTrapSound)
    (if (Variables|ActionDONOTEDITTHOSE|GetHasFired)
      (CallFunction|ShellEjecting)
      (Variables|ActionDONOTEDITTHOSE|SetHasFired false))
    (else
      (CallFunction|AmmAnim)
      (CallFunction|LeverAnim)
      (Variables|ActionDONOTEDITTHOSE|SetTrapClosed true)
      (CallFunction|PlayTrapSound))))

(event OnInteractBoxClient(Pavlov_Reload)
  (params (InteractType :type EInteractType%20Enum :default "Grabbed") (HandProxy :type Pavlov%20Hand%20Proxy%20Object%20Reference) (InteractBox :type Pavlov%20Interact%20Box%20Object%20Reference))
  ;[1 1 1] Interaction Pavlov Replication
  (Class|PavlovHandProxy|ReplicateInteractServer HandProxy InteractType InteractBox))

(event OnInteractBoxClient(Pavlov_RotateLeft)
  (params (InteractType :type EInteractType%20Enum :default "Grabbed") (HandProxy :type Pavlov%20Hand%20Proxy%20Object%20Reference) (InteractBox :type Pavlov%20Interact%20Box%20Object%20Reference))
  ;[1 1 1] Interaction Pavlov Replication
  (Class|PavlovHandProxy|ReplicateInteractServer HandProxy InteractType InteractBox))

(event OnInteractBoxClient(Pavlov_RotateRight)
  (params (InteractType :type EInteractType%20Enum :default "Grabbed") (HandProxy :type Pavlov%20Hand%20Proxy%20Object%20Reference) (InteractBox :type Pavlov%20Interact%20Box%20Object%20Reference))
  ;[1 1 1] Interaction Pavlov Replication
  (Class|PavlovHandProxy|ReplicateInteractServer HandProxy InteractType InteractBox))

(event Custom|FireLoop
  ;[1 0.1094 0.1094] DEBUG
  (CallFunction|TestreloadClient)
  (CallFunction|TesttrapClient)
  (Utilities|FlowControl|Delay 1.0)
  (CallFunction|Testfire))

(event Custom|PlayFireFX
  (bind _pak_cannon (Variables|Components|GetPak_Cannon))
  (bind _returnvalue (Transformation|GetSocketTransform _pak_cannon "FireSocket" "RTS_World"))
  ;[1 0.823 0.4892] FX
  (Effects|SpawnEmitteratLocation (Variables|EditableVariables|GetFiringEmitter) (.location _returnvalue) (.rotation _returnvalue) "0.500000,0.500000,0.500000")
  (Audio|PlaySoundatLocation (Variables|EditableVariables|GetFiringSound) (.location _returnvalue) "0, 0, 0" 1.0 1.0 0.0 "/Game/CustomMaps/UGC2436162648/Artillery/Common/Sound/SA_Antitankgun.SA_Antitankgun" 0 0))

(event Custom|FireAnimation
  (bind _pak_cannon (Variables|Components|GetPak_Cannon))
  ;[0.2874 0.9131 1] Fire Animation
  (bind _newtrack_1 (Timeline|Timeline_3 PlayFromStart)
    (:Update
      (Transformation|AddLocalOffset _pak_cannon (Math|Vector|Lerp(Vector) "0, 0, 0" "0.000000,-4.000000, 0" _newtrack_1) false false))
    (:Finished
      (Transformation|SetRelativeLocation _pak_cannon (Variables|AnimationDONOTEDITTHOSE|GetCannonInitLocation) false false))))

(event Custom|RotateWheelYDown
  ;[0.2874 0.9131 1] Wheels Animation
  (Transformation|AddLocalRotation (Variables|Components|GetPak_LeftYawWheel) (Math|Rotator|MakeRotator 0.0 (* (Variables|AnimationDONOTEDITTHOSE|GetWheelSpeed) -1.0) 0.0) false false))

(event Custom|LeverAnim
  ;[0.2874 0.9131 1] Reload Animation
  ;;[1 1 1] Lever
  (Timeline|Timeline_1 PlayFromStart
    (:Update
      (Transformation|AddLocalRotation (Variables|Components|GetPak_Lever) "0,1.000000, 0" false false))))

(event Custom|SetDestroyedHidden
  ;[1 0.1269 0] Damage
  (Development|SetHiddeninGame (Variables|Default|GetPak_Destroyed) true false))

(event Custom|LeverAnimUnload
  (bind _pak_lever (Variables|Components|GetPak_Lever))
  ;[0.2874 0.9131 1] Reload Animation
  ;;[1 1 1] Lever
  (Timeline|Timeline_2 PlayFromStart
    (:Update
      (Transformation|AddLocalRotation _pak_lever "0,-1.000000, 0" false false))
    (:Finished
      (Transformation|SetRelativeRotation _pak_lever (Variables|AnimationDONOTEDITTHOSE|GetLeverInitRotation) false false))))

(event Custom|ActivateFireLoop
  ;[1 0.1094 0.1094] DEBUG
  (bind _returnvalue (Utilities|Time|SetTimerbyEvent (delegate Custom|FireLoop) 2.0 true)))

(event Custom|DeactivateFireLoop
  ;[1 0.1094 0.1094] DEBUG
  (Utilities|Time|PauseTimerbyHandle (stale Custom|ActivateFireLoop _returnvalue)))

(event Custom|ReactivateFireLoop
  ;[1 0.1094 0.1094] DEBUG
  (Utilities|Time|UnpauseTimerbyHandle (stale Custom|ActivateFireLoop _returnvalue)))

(event Custom|ShellEjecting
  (bind _pavlov_loading (Variables|Components|GetPavlov_Loading))
  ;[0.2874 0.9131 1] Shell Emitter
  (Utilities|FlowControl|Delay 0.5)
  (Rendering|SetVisibility (Variables|Components|GetShellCaseMesh) false true)
  (Effects|SpawnEmitteratLocation "/Game/CustomMaps/UGC2436162648/Artillery/Common/Particles/PS_ShellParticle.PS_ShellParticle" (Transformation|GetWorldLocation _pavlov_loading) (Transformation|GetWorldRotation _pavlov_loading)))

(event Custom|SetAlternateMaterial
  (bind _pak_cannon (Variables|Components|GetPak_Cannon))
  ;[1 1 1] Alternate Texture
  (Rendering|Material|SetMaterial _pak_cannon 1 "/Game/CustomMaps/UGC2436162648/Artillery/Pak_40/Materials/M_GermanPak40_Alternate1.M_GermanPak40_Alternate1")
  (Rendering|Material|SetMaterial _pak_cannon 2 "/Game/CustomMaps/UGC2436162648/Artillery/Pak_40/Materials/M_GermanPak40_Alternate2.M_GermanPak40_Alternate2")
  (Rendering|Material|SetMaterial (Variables|Default|GetPak_Destroyed) 1 "/Game/CustomMaps/UGC2436162648/Artillery/Pak_40/Materials/M_GermanPak40_Alternate1.M_GermanPak40_Alternate1")
  (Rendering|Material|SetMaterial (Variables|Components|GetPak_Right_YawWheel) 1 "/Game/CustomMaps/UGC2436162648/Artillery/Pak_40/Materials/M_GermanPak40_Alternate2.M_GermanPak40_Alternate2")
  (Rendering|Material|SetMaterial (Variables|Components|GetPak_Lever) 0 "/Game/CustomMaps/UGC2436162648/Artillery/Pak_40/Materials/M_GermanPak40_Alternate2.M_GermanPak40_Alternate2"))

(event Custom|Respawn
  ;[1 0.1269 0] Damage
  (if (!= (Variables|Health|GetRespawnDelay) -1.0)
    (Utilities|FlowControl|Delay (Variables|Health|GetRespawnDelay))
    (Variables|Health|SetCurrentHealth (Variables|Health|GetMaxHealth))
    (CallFunction|UnHideDestroyed)))

(event Custom|PlayShellLoadSound
  ;[1 0.823 0.4892] FX
  (Audio|PlaySoundatLocation (Variables|EditableVariables|GetShellLoadingSound) (.location (Transformation|GetSocketTransform (Variables|Components|GetPak_Trap) "None" "RTS_World")) "0, 0, 0" 1.0 1.0 0.0 "/Game/CustomMaps/UGC2436162648/Artillery/Common/Sound/SA_Close.SA_Close" 0 0))

(event Custom|AutoStopTimer
  ;[0.8025 1 0.6847] Controls
  ;;[1 1 1] AutoStop Security
  (Variables|MovementDONOTEDITTHOSE|SetDR_R_Stop true)
  (Variables|MovementDONOTEDITTHOSE|SetGB_UP_Stop true)
  (Variables|MovementDONOTEDITTHOSE|SetDR_L_Stop true)
  (Variables|MovementDONOTEDITTHOSE|SetGB_DO_Stop true))

(event Custom|testtrap_Client
  ;[1 0.5647 0.7758] Loading
  (if (Variables|ActionDONOTEDITTHOSE|GetTrapClosed)
    (Variables|ActionDONOTEDITTHOSE|SetHasEmptyShell false)
    (CallFunction|UnloadAmmAnim)
    (CallFunction|LeverAnimUnload)
    (Variables|ActionDONOTEDITTHOSE|SetTrapClosed false)
    (CallFunction|PlayTrapSound)
    (if (Variables|ActionDONOTEDITTHOSE|GetHasFired)
      (CallFunction|ShellEjecting)
      (Variables|ActionDONOTEDITTHOSE|SetHasFired false))
    (else
      (CallFunction|AmmAnim)
      (CallFunction|LeverAnim)
      (Variables|ActionDONOTEDITTHOSE|SetTrapClosed true)
      (CallFunction|PlayTrapSound))))

(event Custom|testfire
  (bind _pak_cannon (Variables|Components|GetPak_Cannon))
  (bind _returnvalue (Transformation|GetSocketTransform _pak_cannon "FireSocket" "RTS_World"))
  ;[1 0.5647 0.7758] Firing
  (if (Variables|ActionDONOTEDITTHOSE|GetIsLoaded)
    (if (Variables|ActionDONOTEDITTHOSE|GetTrapClosed)
      (CallFunction|PlayFireFX)
      (CallFunction|FireAnimation)
      (Variables|ActionDONOTEDITTHOSE|SetIsLoaded false)
      (Variables|ActionDONOTEDITTHOSE|SetHasFired true)
      (Variables|ActionDONOTEDITTHOSE|SetHasEmptyShell true)
      (Game|SpawnActorfromClass "/Game/CustomMaps/UGC2436162648/Artillery/Common/Projectiles/BP_ArtilleryProjectile.BP_ArtilleryProjectile_C" (Math|Transform|MakeTransform (.location _returnvalue) (.rotation _returnvalue) "0.180000,0.180000,0.180000") "AlwaysSpawn" 0 "/Game/CustomMaps/UGC2436162648/Artillery/Common/Sound/grenade_explo_Cue.grenade_explo_Cue" "/Game/CustomMaps/UGC2436162648/Artillery/Common/Sound/Explosiondistant_Cue.Explosiondistant_Cue" "/Game/CustomMaps/UGC2436162648/Artillery/Common/Decals/T_Impact.T_Impact" (Game|GetInstigator (Components|GetOwner (stale OnInteractBoxServer(Pavlov_Fire) HandProxy)))))))

(event Custom|testrotatedown
  (bind _pak_rail (Variables|Components|GetPak_Rail))
  ;[0.8025 1 0.6847] Controls
  ;;[1 1 1] Y Movement
  (if (Variables|MovementDONOTEDITTHOSE|GetGB_DO_Stop)
    (CallFunction|AutoStop)
    (if (Variables|MovementDONOTEDITTHOSE|GetGB_UP_Stop)
      _
      (else
        (Variables|MovementDONOTEDITTHOSE|SetGB_UP_Stop true)))
    (Variables|MovementDONOTEDITTHOSE|SetGB_DO_Stop false)
    (if (not (Variables|MovementDONOTEDITTHOSE|GetGB_DO_Stop)) :!label _label
      (if (>= (.roll (Variables|/Script/Engine.SceneComponent|GetRelativeRotation _pak_rail)) 2.0)
        (Variables|MovementDONOTEDITTHOSE|SetGB_DO_Stop true)
        (else
          (Transformation|AddLocalRotation _pak_rail (Math|Rotator|MakeRotator (Variables|MovementDONOTEDITTHOSE|GetGunBarrelYDegree) 0.0 0.0) false false)
          (Utilities|FlowControl|Delay (Variables|MovementDONOTEDITTHOSE|GetGunBarrelYSpeed))
          (CallFunction|RotateWheelYDown)
          (CallFunction|PlayRotationSound)
          (goto _label))))
    (else
      (Variables|MovementDONOTEDITTHOSE|SetGB_DO_Stop true)
      (Variables|MovementDONOTEDITTHOSE|SetGB_UP_Stop true))))

(event Custom|testrotateup
  (bind _pak_rail (Variables|Components|GetPak_Rail))
  ;[0.8025 1 0.6847] Controls
  ;;[1 1 1] Y Movement
  (if (Variables|MovementDONOTEDITTHOSE|GetGB_UP_Stop)
    (CallFunction|AutoStop)
    (if (Variables|MovementDONOTEDITTHOSE|GetGB_DO_Stop)
      _
      (else
        (Variables|MovementDONOTEDITTHOSE|SetGB_DO_Stop true)))
    (Variables|MovementDONOTEDITTHOSE|SetGB_UP_Stop false)
    (if (not (Variables|MovementDONOTEDITTHOSE|GetGB_UP_Stop)) :!label _label
      (if (<= (.roll (Variables|/Script/Engine.SceneComponent|GetRelativeRotation _pak_rail)) -7.0)
        (Variables|MovementDONOTEDITTHOSE|SetGB_UP_Stop true)
        (else
          (Transformation|AddLocalRotation _pak_rail (Math|Rotator|MakeRotator (* (Variables|MovementDONOTEDITTHOSE|GetGunBarrelYDegree) -1.0) 0.0 0.0) false false)
          (Utilities|FlowControl|Delay (Variables|MovementDONOTEDITTHOSE|GetGunBarrelYSpeed))
          (CallFunction|RotateWheelYUp)
          (CallFunction|PlayRotationSound)
          (goto _label))))
    (else
      (Variables|MovementDONOTEDITTHOSE|SetGB_UP_Stop true)
      (Variables|MovementDONOTEDITTHOSE|SetGB_DO_Stop true))))

(event Custom|testrotateleft
  (bind _pak_turret (Variables|Components|GetPak_Turret))
  ;[0.8025 1 0.6847] Controls
  ;;[1 1 1] Z Movement
  (if (Variables|MovementDONOTEDITTHOSE|GetDR_L_Stop)
    (CallFunction|AutoStop)
    (if (Variables|MovementDONOTEDITTHOSE|GetDR_R_Stop)
      _
      (else
        (Variables|MovementDONOTEDITTHOSE|SetDR_R_Stop true)))
    (Variables|MovementDONOTEDITTHOSE|SetDR_L_Stop false)
    (if (not (Variables|MovementDONOTEDITTHOSE|GetDR_L_Stop)) :!label _label
      (if (<= (.yaw (Variables|/Script/Engine.SceneComponent|GetRelativeRotation _pak_turret)) -25.0)
        (Variables|MovementDONOTEDITTHOSE|SetDR_L_Stop true)
        (else
          (Transformation|AddLocalRotation _pak_turret (Math|Rotator|MakeRotator 0.0 0.0 (* (Variables|MovementDONOTEDITTHOSE|GetDockRotateZDegree) -1.0)) false false)
          (Utilities|FlowControl|Delay (Variables|MovementDONOTEDITTHOSE|GetDockRotateZSpeed))
          (CallFunction|RotateWheelZRight)
          (CallFunction|PlayRotationSound)
          (goto _label))))
    (else
      (Variables|MovementDONOTEDITTHOSE|SetDR_L_Stop true)
      (Variables|MovementDONOTEDITTHOSE|SetDR_R_Stop true))))

(event Custom|HideDestroyed
  (bind _pak_dock (Variables|Components|GetPak_Dock))
  ;[1 0.1269 0] Damage
  (Development|SetHiddeninGame _pak_dock true true)
  (Collision|SetCollisionEnabled _pak_dock "NoCollision")
  (bind _returnvalue (Class|GameplayStatics|SpawnDecalAttached "/Game/CustomMaps/UGC2436162648/Artillery/Common/Decals/T_Impact.T_Impact" "1000.000000,1000.000000,1000.000000" (Variables|Default|GetPak_Destroyed) "None" "0, 0, 0" "-90.000000,0.000000,0.000000" "KeepRelativeOffset" (Variables|Health|GetRespawnDelay)))
  (Variables|Default|SetDamagedDecal _returnvalue)
  (Development|SetHiddeninGame (Variables|Default|GetPak_Destroyed) false true)
  (Collision|SetCollisionEnabled (Variables|Default|GetPak_Destroyed) "QueryAndPhysics"))

(event Custom|InitialRotation
  ;[0.6417 0.5249 1] BeginPlay
  (Utilities|FlowControl|Delay 0.2)
  (CallFunction|Testrotateright)
  (CallFunction|Testrotateup)
  (Utilities|FlowControl|Delay 1e+01)
  (CallFunction|Testrotateright)
  (CallFunction|Testrotateup))

(event Custom|testdebug_fireloop
  ;[1 0.1094 0.1094] DEBUG
  (CallFunction|ActivateFireLoop)
  (CallFunction|ReactivateFireLoop))

(event Custom|testreload_client
  ;[1 0.5647 0.7758] Loading
  (Utilities|CanReload?
    (:Yes
      (Variables|ActionDONOTEDITTHOSE|SetIsLoaded true)
      (CallFunction|PlayShellLoadSound))))

(event Custom|RotateWheelYUp
  ;[0.2874 0.9131 1] Wheels Animation
  (Transformation|AddLocalRotation (Variables|Components|GetPak_LeftYawWheel) (Math|Rotator|MakeRotator 0.0 (Variables|AnimationDONOTEDITTHOSE|GetWheelSpeed) 0.0) false false))

(event Custom|PlayRotationSound
  ;[1 0.823 0.4892] FX
  (Utilities|FlowControl|Delay 0.5)
  (Audio|PlaySoundatLocation (Variables|EditableVariables|GetRotationSound) (Transformation|GetSocketLocation (Variables|Components|GetPak_Right_YawWheel) "None") "0, 0, 0" 0.25 -1.0 0.0 "/Game/CustomMaps/UGC2436162648/Artillery/Common/Sound/SA_Close.SA_Close" 0 0))

(event Custom|RotateWheelZLeft
  ;[0.2874 0.9131 1] Wheels Animation
  (Transformation|AddLocalRotation (Variables|Components|GetPak_Right_YawWheel) (Math|Rotator|MakeRotator 0.0 (Variables|AnimationDONOTEDITTHOSE|GetWheelSpeed) 0.0) false false))

(event Custom|testdebug_client
  ;[1 0.1094 0.1094] DEBUG
  (Utilities|FlowControl|MultiGate false true -1
    (:Out%200
      (Variables|Debug|SetDEBUG true)
      (Variables|Debug|SetHiddeBoxes false))
    (:Out%201
      (Variables|Debug|SetDEBUG false)
      (Variables|Debug|SetHiddeBoxes true)))
  (Development|SetHiddeninGame (Variables|Components|GetPavlov_Loading) (Variables|Debug|GetHiddeBoxes) false)
  (Transformation|SetRelativeScale3D (Variables|Components|GetFireDirectionArrow) "4000.000000,2.000000,2.000000"))

(event Custom|UnHideDestroyed
  (bind _damageddecal (Variables|Default|GetDamagedDecal))
  ;[1 0.1269 0] Damage
  (Development|SetHiddeninGame (Variables|Components|GetPak_Dock) false true)
  (Utilities|IsValid _damageddecal
    (:Is%20Valid
      (Components|DestroyComponent _damageddecal))
    (:Is%20Not%20Valid
      _))
  (Collision|SetCollisionEnabled (Variables|Components|GetPak_Dock) "QueryAndPhysics")
  (Collision|SetCollisionEnabled (Variables|Components|GetPavlov_Fire) "QueryOnly")
  (Collision|SetCollisionEnabled (Variables|Default|GetPak_Destroyed) "NoCollision")
  (Development|SetHiddeninGame (Variables|Default|GetPak_Destroyed) true false))

(event Custom|testdebug_stopfireloop
  ;[1 0.1094 0.1094] DEBUG
  (CallFunction|DeactivateFireLoop))

(event Custom|EnableInput_Client
  ;[0.6417 0.5249 1] BeginPlay
  (Input|EnableInput (Game|GetPlayerController 0)))

(event Custom|testrotateright
  ;[0.8025 1 0.6847] Controls
  ;;[1 1 1] Z Movement
  (if (Variables|MovementDONOTEDITTHOSE|GetDR_R_Stop)
    (CallFunction|AutoStop)
    (if (Variables|MovementDONOTEDITTHOSE|GetDR_L_Stop)
      _
      (else
        (Variables|MovementDONOTEDITTHOSE|SetDR_L_Stop true)))
    (Variables|MovementDONOTEDITTHOSE|SetDR_R_Stop false)
    (if (not (Variables|MovementDONOTEDITTHOSE|GetDR_R_Stop)) :!label _label
      (if (>= (.yaw (Variables|/Script/Engine.SceneComponent|GetRelativeRotation (Variables|Components|GetPak_Turret))) 25.0)
        (Variables|MovementDONOTEDITTHOSE|SetDR_R_Stop true)
        (else
          (Transformation|AddLocalRotation (Variables|Components|GetPak_Turret) (Math|Rotator|MakeRotator 0.0 0.0 (Variables|MovementDONOTEDITTHOSE|GetDockRotateZDegree)) false false)
          (Utilities|FlowControl|Delay (Variables|MovementDONOTEDITTHOSE|GetDockRotateZSpeed))
          (CallFunction|RotateWheelZLeft)
          (CallFunction|PlayRotationSound)
          (goto _label))))
    (else
      (Variables|MovementDONOTEDITTHOSE|SetDR_R_Stop true)
      (Variables|MovementDONOTEDITTHOSE|SetDR_L_Stop true))))

(event Custom|RotateWheelZRight
  ;[0.2874 0.9131 1] Wheels Animation
  (Transformation|AddLocalRotation (Variables|Components|GetPak_Right_YawWheel) (Math|Rotator|MakeRotator 0.0 (Variables|AnimationDONOTEDITTHOSE|GetWheelSpeed) 0.0) false false))

(event Custom|PlayTrapSound
  ;[1 0.823 0.4892] FX
  (Audio|PlaySoundatLocation (Variables|EditableVariables|GetTrapSound) (.location (Transformation|GetSocketTransform (Variables|Components|GetPak_Trap) "None" "RTS_World")) "0, 0, 0" 1.0 1.0 0.0 "/Game/CustomMaps/UGC2436162648/Artillery/Common/Sound/SA_Close.SA_Close" 0 0))

(event Custom|AutoStop
  ;[0.8025 1 0.6847] Controls
  ;;[1 1 1] AutoStop Security
  (Utilities|Time|SetTimerbyEvent (delegate Custom|AutoStopTimer) 15.0))

(event Custom|AmmAnim
  ;[0.2874 0.9131 1] Reload Animation
  ;;[1 1 1] Ammunition Trap
  (bind _newtrack_1 (Timeline|Timeline_0 PlayFromStart)
    (:Update
      (Transformation|AddLocalOffset (Variables|Components|GetPak_Trap) (Math|Vector|Lerp(Vector) "0, 0, 0" "-0.550000,0.000000, 0" _newtrack_1) false false))))

(event Custom|UnloadAmmAnim
  (bind _pak_trap (Variables|Components|GetPak_Trap))
  ;[0.2874 0.9131 1] Reload Animation
  ;;[1 1 1] Ammunition Trap
  (bind _newtrack_1 (Timeline|Timeline_4 PlayFromStart)
    (:Update
      (Transformation|AddLocalOffset _pak_trap (Math|Vector|Lerp(Vector) "0, 0, 0" "0.550000,0.000000, 0" _newtrack_1) false false))
    (:Finished
      (Transformation|SetRelativeLocation _pak_trap (Variables|AnimationDONOTEDITTHOSE|GetTropInitLocation) false false))))

(event EventBeginPlay
  ;[0.6417 0.5249 1] BeginPlay
  (Utilities|FlowControl|Delay 2.0)
  (Networking|SwitchHasAuthority
    (:Authority
      (Variables|Health|SetCurrentHealth (Variables|Health|GetMaxHealth))
      (if (Variables|Debug|GetInputEnabled?)
        (CallFunction|EnableInputClient))
      (if (Variables|Default|GetUseGreyTexture)
        (CallFunction|SetAlternateMaterial))
      (Variables|ActionDONOTEDITTHOSE|SetIsLoaded true)
      (Variables|ActionDONOTEDITTHOSE|SetTrapClosed false)
      (if (Variables|Debug|GetDEBUG_FireLoopBegin)
        (CallFunction|ActivateFireLoop))
      (if (Variables|Debug|GetDEBUG_InitialRotation)
        (CallFunction|InitialRotation)))
    (:Remote
      (Utilities|FlowControl|Delay 1.0)
      (if (Variables|Default|GetUseGreyTexture)
        (CallFunction|SetAlternateMaterial)))))

(event Game|Damage|EventAnyDamage
  (params (Damage :type Float%20%28single-precision%29) (DamageType :type Damage%20Type%20Object%20Reference) (InstigatedBy :type Controller%20Object%20Reference) (DamageCauser :type Actor%20Object%20Reference))
  (bind _returnvalue (Utilities|GetDisplayName DamageCauser))
  (bind _returnvalue_2 (Utilities|String|StartsWith _returnvalue "Bullet_Tank"))
  (bind _returnvalue_3 (Utilities|String|StartsWith _returnvalue "Shell_"))
  ;[1 0.1269 0] Damage
  (if (Math|Boolean|ORBoolean (Utilities|String|StartsWith _returnvalue "Rocket") _returnvalue_2 (Utilities|String|StartsWith _returnvalue "Grenade_") _returnvalue_3 (Utilities|String|StartsWith _returnvalue "BP_ArtilleryProjectile"))
    (if (or _returnvalue_2 _returnvalue_3)
      ;;[1 1 1] Tank damage = 10
      ;; -> Multiply value to increase realism
      (Variables|Health|SetCurrentHealth (- (Variables|Health|GetCurrentHealth) (* Damage 2e+01)))
      (else
        (Variables|Health|SetCurrentHealth (- (Variables|Health|GetCurrentHealth) Damage))))
    (if (<= (Variables|Health|GetCurrentHealth) 0.0)
      (CallFunction|HideDestroyed)
      (CallFunction|Respawn))))

(event Input|KeyboardEvents|9
  (params (Key :type Key%20Structure))
  ;[1 0.1094 0.1094] DEBUG
  ;;[1 1 1] Editor Controls
  (:Pressed
    (CallFunction|TestdebugStopfireloop)))

(event Input|KeyboardEvents|8
  (params (Key :type Key%20Structure))
  ;[1 0.1094 0.1094] DEBUG
  ;;[1 1 1] Editor Controls
  (:Pressed
    (CallFunction|TestdebugFireloop)))

(event Input|KeyboardEvents|Up
  (params (Key :type Key%20Structure))
  ;[1 0.1094 0.1094] DEBUG
  ;;[1 1 1] Editor Controls
  (:Pressed
    (CallFunction|Testrotateup)))

(event Input|KeyboardEvents|Down
  (params (Key :type Key%20Structure))
  ;[1 0.1094 0.1094] DEBUG
  ;;[1 1 1] Editor Controls
  (:Pressed
    (CallFunction|Testrotatedown)))

(event Input|KeyboardEvents|0
  (params (Key :type Key%20Structure))
  ;[1 0.1094 0.1094] DEBUG
  ;;[1 1 1] Editor Controls
  (:Pressed
    (CallFunction|TestdebugClient)))

(event Input|KeyboardEvents|1
  (params (Key :type Key%20Structure))
  ;[1 0.1094 0.1094] DEBUG
  ;;[1 1 1] Editor Controls
  (:Pressed
    (CallFunction|Testfire)))

(event Input|KeyboardEvents|2
  (params (Key :type Key%20Structure))
  ;[1 0.1094 0.1094] DEBUG
  ;;[1 1 1] Editor Controls
  (:Pressed
    (CallFunction|TesttrapClient)))

(event Input|KeyboardEvents|3
  (params (Key :type Key%20Structure))
  ;[1 0.1094 0.1094] DEBUG
  ;;[1 1 1] Editor Controls
  (:Pressed
    (CallFunction|TestreloadClient)))

(event Input|KeyboardEvents|Left
  (params (Key :type Key%20Structure))
  ;[1 0.1094 0.1094] DEBUG
  ;;[1 1 1] Editor Controls
  (:Pressed
    (CallFunction|Testrotateleft)))

(event Input|KeyboardEvents|Right
  (params (Key :type Key%20Structure))
  ;[1 0.1094 0.1094] DEBUG
  ;;[1 1 1] Editor Controls
  (:Pressed
    (CallFunction|Testrotateright)))

(fn ConstructionScript)

(fn OnRepIsLoaded
  (bind _shellmesh (Variables|Components|GetShellMesh))
  (bind _shellcasemesh (Variables|Components|GetShellCaseMesh))
  (if (Variables|ActionDONOTEDITTHOSE|GetIsLoaded)
    (Rendering|SetVisibility _shellmesh true true)
    (Rendering|SetVisibility _shellcasemesh false true)
    (else
      (Rendering|SetVisibility _shellmesh false true)
      (Rendering|SetVisibility _shellcasemesh true true))))