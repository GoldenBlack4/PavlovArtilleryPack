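; Actor that stands in as the wreck of a destroyed artillery piece from the artillery pack.
; SpawnDestroyed checks the source object's class against five gun types and adds a matching static mesh component, with alternate materials for some guns when requested.
; It attaches an impact decal to the mesh, then destroys itself after the respawn delay unless that delay is -1.
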(event Custom|SpawnDestroyed
  (params (UseAlternateTexture :type Boolean) (Object :type Object%20Object%20Reference) (RespawnDelay :type Float%20%28single-precision%29))
  (bind _returnvalue (Utilities|GetClass Object))
  (Variables|Default|SetUseAlternateTexture UseAlternateTexture)
  (Variables|Default|SetRespawnDelay RespawnDelay)
  (if (== _returnvalue "/Game/CustomMaps/UGC2436162648/ArtilleryPack/Pak_40/BPM_Pak40.BPM_Pak40_C")
    (bind _returnvalue_2 (AddComponent|AddStaticMeshComponent false))
    (if (Variables|Default|GetUseAlternateTexture)
      (Rendering|Material|SetMaterial _returnvalue_2 1 "/Game/CustomMaps/UGC2436162648/ArtilleryPack/Pak_40/Materials/M_GermanPak40_Alternate1.M_GermanPak40_Alternate1")
      (Rendering|Material|SetMaterial _returnvalue_2 0 "/Game/CustomMaps/UGC2436162648/ArtilleryPack/Pak_40/Materials/M_GermanPak40_Alternate2.M_GermanPak40_Alternate2"))
    (Class|GameplayStatics|SpawnDecalAttached "/Game/CustomMaps/UGC2436162648/ArtilleryPack/Common/Decals/T_Impact.T_Impact" "1000.000000,1000.000000,1000.000000" _returnvalue_2 "None" "0, 0, 0" "-90.000000,0.000000,0.000000" "KeepRelativeOffset" 0.0)
    (if (not (== (Variables|Default|GetRespawnDelay) -1.0)) :!label _label
      (Utilities|FlowControl|Delay (Variables|Default|GetRespawnDelay))
      (Actor|DestroyActor))
    (elif (== _returnvalue "/Game/CustomMaps/UGC2436162648/ArtilleryPack/Flak_88/BPC_Flak88.BPC_Flak88_C")
      (bind _returnvalue_3 (AddComponent|AddStaticMeshComponent false))
      (Class|GameplayStatics|SpawnDecalAttached "/Game/CustomMaps/UGC2436162648/ArtilleryPack/Common/Decals/T_Impact.T_Impact" "1000.000000,1000.000000,1000.000000" _returnvalue_3 "None" "0, 0, 0" "-90.000000,0.000000,0.000000" "KeepRelativeOffset" 0.0)
      (goto _label)
      (elif (== _returnvalue "/Game/CustomMaps/UGC2436162648/ArtilleryPack/QF6/BPC_QF6.BPC_QF6_C")
        (bind _returnvalue_4 (AddComponent|AddStaticMeshComponent false))
        (if (Variables|Default|GetUseAlternateTexture)
          (Rendering|Material|SetMaterial _returnvalue_4 1 "/Game/CustomMaps/UGC2436162648/ArtilleryPack/QF6/Materials/QF6_BaseColor_alternate.QF6_BaseColor_alternate"))
        (Class|GameplayStatics|SpawnDecalAttached "/Game/CustomMaps/UGC2436162648/ArtilleryPack/Common/Decals/T_Impact.T_Impact" "1000.000000,1000.000000,1000.000000" _returnvalue_4 "None" "0, 0, 0" "-90.000000,0.000000,0.000000" "KeepRelativeOffset" 0.0)
        (goto _label)
        (elif (== _returnvalue "/Game/CustomMaps/UGC2436162648/ArtilleryPack/ZiS/BPC_ZiS2.BPC_ZiS2_C")
          (bind _returnvalue_5 (AddComponent|AddStaticMeshComponent false))
          (if (Variables|Default|GetUseAlternateTexture)
            (Rendering|Material|SetMaterial _returnvalue_5 1 "/Game/CustomMaps/UGC2436162648/ArtilleryPack/ZiS/Materials/MI_Zis2_01_alternate.MI_Zis2_01_alternate")
            (Rendering|Material|SetMaterial _returnvalue_5 0 "/Game/CustomMaps/UGC2436162648/ArtilleryPack/ZiS/Materials/MI_Zis2_02_alternate.MI_Zis2_02_alternate"))
          (Class|GameplayStatics|SpawnDecalAttached "/Game/CustomMaps/UGC2436162648/ArtilleryPack/Common/Decals/T_Impact.T_Impact" "1000.000000,1000.000000,1000.000000" _returnvalue_5 "None" "0, 0, 0" "-90.000000,0.000000,0.000000" "KeepRelativeOffset" 0.0)
          (goto _label)
          (elif (== _returnvalue "/Game/CustomMaps/UGC2436162648/ArtilleryPack/Pak_43/BPC_Pak43.BPC_Pak43_C")
            (bind _returnvalue_6 (AddComponent|AddStaticMeshComponent false))
            (if (Variables|Default|GetUseAlternateTexture)
              (Rendering|Material|SetMaterial _returnvalue_6 0 "/Game/CustomMaps/UGC2436162648/ArtilleryPack/Pak_43/Materials/M_Pak43_alternate.M_Pak43_alternate"))
            (Class|GameplayStatics|SpawnDecalAttached "/Game/CustomMaps/UGC2436162648/ArtilleryPack/Common/Decals/T_Impact.T_Impact" "1000.000000,1000.000000,1000.000000" _returnvalue_6 "None" "0, 0, 0" "-90.000000,0.000000,0.000000" "KeepRelativeOffset" 0.0)
            (goto _label)))))))

(fn ConstructionScript)