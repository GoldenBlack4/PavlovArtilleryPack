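; Spawner actor that keeps a smoke artillery shell available at its placed location in a Pavlov custom map.
; On BeginPlay it removes its placeholder shell mesh, then runs an endless server-only loop.
; The loop polls while the spawned shell is still valid; once it is gone, it waits RespawnDelay and spawns a replacement through the game logic's SpawnItemWRef, retrying if that fails.
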(event EventBeginPlay
  (bind _returnvalue (Class|PavlovLibrary|GetGameLogic))
  (Components|DestroyComponent (Variables|Default|GetShellMesh_Smoke))
  (Networking|SwitchHasAuthority :!label _label
    (:Authority
      (Utilities|IsValid (Variables|Default|GetSpawnedPavlovShell)
        (:Is%20Valid
          (Utilities|FlowControl|Delay 2.0)
          (goto _label))
        (:Is%20Not%20Valid
          (Utilities|FlowControl|Delay (Variables|Default|GetRespawnDelay))
          (Utilities|IsValid _returnvalue
            (:Is%20Valid
              (bind (_bsuccessful _item) (Class|PavlovGameLogic|SpawnItemWRef _returnvalue (Utilities|Struct|MakePavlovItemSpawnParams "artilleryshell_smoke" 0 false false 0 true (Transformation|GetActorTransform) false true)))
              (if _bsuccessful
                (Variables|Default|SetSpawnedPavlovShell _item)
                (goto _label)
                (else
                  (goto _label))))
            (:Is%20Not%20Valid
              (goto _label))))))))

(fn ConstructionScript)