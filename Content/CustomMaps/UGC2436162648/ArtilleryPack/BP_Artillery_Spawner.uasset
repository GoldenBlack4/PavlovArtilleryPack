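; Placeable spawner for the artillery pack that spawns a selected anti-tank gun, passing on its settings, then destroys itself.
; Construction script previews the gun through a data-table-driven child actor, removed at BeginPlay.
; On the server, PushMacro polls every five seconds in Push modes until the objective matches (ID -1 skips waiting).
; Outside Push it spawns after InitialSpawnDelay, or self-destructs if marked Push-only.
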(event Custom|SpawnAT
  ;[0.7163 1 0.6135] Spawn AT
  (Utilities|FlowControl|Delay (Variables|Required|GetInitialSpawnDelay))
  (switch Utilities|FlowControl|Switch|SwitchonE_Artillery (Variables|Required|GetArtillery%20to%20spawn)
    (:NewEnumerator0
      (Game|SpawnActorfromClass "/Game/CustomMaps/UGC2436162648/ArtilleryPack/Flak_88/BPC_Flak88.BPC_Flak88_C" (Variables|Donotedit|GetSpawnTransform) "AlwaysSpawn" 0 (Variables|DEBUG|GetDEBUG_InputEnabled) (Variables|Required|GetRespawnDelay) (Variables|Required|GetMaxHealth) (Variables|Required|GetNoRespawn) (Variables|Required|GetOnlySpawnInPush) (Variables|FX|GetFiringEmitter) (Variables|FX|GetFiringSound) (Variables|FX|GetBreechSound) (Variables|FX|GetShellLoadingSound) (Variables|Required|GetUseAlternateTexture) (Variables|Required|GetUseSpawnableCrates) (Variables|Required|GetAllowTrailerMode) (Variables|Required|GetSensitivityMultiplier) (Variables|Required|GetArtillery%20to%20spawn) (Variables|Required|GetPushObjectiveID) (Variables|Required|GetNoSight) 0))
    (:NewEnumerator5
      (Game|SpawnActorfromClass "/Game/CustomMaps/UGC2436162648/ArtilleryPack/Pak_43/BPC_Pak43.BPC_Pak43_C" (Variables|Donotedit|GetSpawnTransform) "AlwaysSpawn" 0 (Variables|DEBUG|GetDEBUG_InputEnabled) (Variables|Required|GetRespawnDelay) (Variables|Required|GetMaxHealth) (Variables|Required|GetNoRespawn) (Variables|Required|GetOnlySpawnInPush) (Variables|FX|GetFiringEmitter) (Variables|FX|GetFiringSound) (Variables|FX|GetBreechSound) (Variables|FX|GetShellLoadingSound) (Variables|Required|GetUseAlternateTexture) (Variables|Required|GetUseSpawnableCrates) (Variables|Required|GetAllowTrailerMode) (Variables|Required|GetSensitivityMultiplier) (Variables|Required|GetArtillery%20to%20spawn) (Variables|Required|GetPushObjectiveID) (Variables|Required|GetNoSight) 0))
    (:NewEnumerator1
      (Game|SpawnActorfromClass "/Game/CustomMaps/UGC2436162648/ArtilleryPack/Pak_40/BPM_Pak40.BPM_Pak40_C" (Variables|Donotedit|GetSpawnTransform) "AlwaysSpawn" 0 (Variables|DEBUG|GetDEBUG_InputEnabled) (Variables|Required|GetRespawnDelay) (Variables|Required|GetMaxHealth) (Variables|Required|GetNoRespawn) (Variables|Required|GetOnlySpawnInPush) (Variables|FX|GetFiringEmitter) (Variables|FX|GetFiringSound) (Variables|FX|GetBreechSound) (Variables|FX|GetShellLoadingSound) (Variables|Required|GetUseAlternateTexture) (Variables|Required|GetUseSpawnableCrates) (Variables|Required|GetAllowTrailerMode) (Variables|Required|GetSensitivityMultiplier) (Variables|Required|GetArtillery%20to%20spawn) (Variables|Required|GetPushObjectiveID) (Variables|Required|GetNoSight) 0))
    (:NewEnumerator2
      (Game|SpawnActorfromClass "/Game/CustomMaps/UGC2436162648/ArtilleryPack/QF6/BPC_QF6.BPC_QF6_C" (Variables|Donotedit|GetSpawnTransform) "AlwaysSpawn" 0 (Variables|DEBUG|GetDEBUG_InputEnabled) (Variables|Required|GetRespawnDelay) (Variables|Required|GetMaxHealth) (Variables|Required|GetNoRespawn) (Variables|Required|GetOnlySpawnInPush) (Variables|FX|GetFiringEmitter) (Variables|FX|GetFiringSound) (Variables|FX|GetBreechSound) (Variables|FX|GetShellLoadingSound) (Variables|Required|GetUseAlternateTexture) (Variables|Required|GetUseSpawnableCrates) (Variables|Required|GetAllowTrailerMode) (Variables|Required|GetSensitivityMultiplier) (Variables|Required|GetArtillery%20to%20spawn) (Variables|Required|GetPushObjectiveID) (Variables|Required|GetNoSight) 0))
    (:NewEnumerator3
      (Game|SpawnActorfromClass "/Game/CustomMaps/UGC2436162648/ArtilleryPack/ZiS/BPC_ZiS2.BPC_ZiS2_C" (Variables|Donotedit|GetSpawnTransform) "AlwaysSpawn" 0 (Variables|DEBUG|GetDEBUG_InputEnabled) (Variables|Required|GetRespawnDelay) (Variables|Required|GetMaxHealth) (Variables|Required|GetNoRespawn) (Variables|Required|GetOnlySpawnInPush) (Variables|FX|GetFiringEmitter) (Variables|FX|GetFiringSound) (Variables|FX|GetBreechSound) (Variables|FX|GetShellLoadingSound) (Variables|Required|GetUseAlternateTexture) (Variables|Required|GetUseSpawnableCrates) (Variables|Required|GetAllowTrailerMode) (Variables|Required|GetSensitivityMultiplier) (Variables|Required|GetArtillery%20to%20spawn) (Variables|Required|GetPushObjectiveID) (Variables|Required|GetNoSight) 0)))
  (Actor|DestroyActor))

(event EventBeginPlay
  ;[1 1 1] Begin Play
  (Utilities|IsValid (Variables|Components|GetAT_Gun)
    (:Is%20Valid
      (Components|DestroyComponent (Variables|Components|GetAT_Gun)))
    (:Is%20Not%20Valid
      _))
  (Networking|SwitchHasAuthority
    (:Authority
      (Variables|Donotedit|SetSpawnTransform (Transformation|GetActorTransform))
      (Utilities|PushMacro :!label _label
        (:Spawn
          (Variables|DoNotEdit|SetWait false)
          (if (Variables|DoNotEdit|GetWait) :!label _label_2
            (Utilities|FlowControl|Delay 5.0)
            (goto _label)
            (else
              (CallFunction|SpawnAT))))
        (:Destroy
          (Actor|DestroyActor))
        (:Wait
          (Variables|DoNotEdit|SetWait true)
          (goto _label_2))))))

(fn ConstructionScript
  (Networking|SwitchHasAuthority
    (:Authority
      (Utilities|FlowControl|Sequence
        (:then_0
          (bind _returnvalue (Utilities|GetDataTableRow "/Game/CustomMaps/UGC2436162648/ArtilleryPack/Common/Blueprints/DTT_Artillery.DTT_Artillery" (Utilities|String|StringToName (Utilities|String|EnumtoString (Variables|Required|GetArtillery%20to%20spawn))))
            (:then
              (ChildActorComponent|SetChildActorClass (Variables|Components|GetAT_Gun) (.Actor (Utilities|Struct|BreakSTR_Artillery _returnvalue))))))
        (:then_1
          (|CallParentFunction))))))